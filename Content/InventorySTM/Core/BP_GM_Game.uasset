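; Game mode that persists a level's added and removed actors in a per-level save slot named after the current level.
; BeginPlay loads the BP_SG_Level save, or creates one if the slot is empty.
; Loaded data drives destruction of removed actors and respawning of added ones from a class-to-transform map, skipping the class of the level's BP_Chest.
; EndPlay writes the save object back to the slot.
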(event `self.ReceiveBeginPlay`
  (bind _returnvalue (`GameplayStatics.GetCurrentLevelName` true))
  (bind _output_get (set `self.Level Data Slot` (`KismetStringLibrary.Concat_StrStr` _returnvalue "_DataGame")))
  (bind _returnvalue_2 (`GameplayStatics.DoesSaveGameExist` _output_get))
  (if _returnvalue_2
    (bind _returnvalue_3 (`GameplayStatics.LoadGameFromSlot` (`self.Level Data Slot`)))
    (bind _asbp_sg_level (cast `/Game/InventorySTM/Blueprints/SaveLoad/BP_SG_Level` _returnvalue_3))
    (bind _output_get_2 (set `self.As BP SG Level` _asbp_sg_level))
    (`GameplayStatics.SaveGameToSlot` _output_get_2 (`self.Level Data Slot`))
    (for _array_element (`/Game/InventorySTM/Blueprints/SaveLoad/BP_SG_Level.ActorsRemoved` (`self.As BP SG Level`))
      (bind _output (`|ConvertAsset` _array_element))
      (`/Engine/EditorBlueprintResources/StandardMacros.IsValid` _output
        (:`Is Valid`
          (`self.K2_DestroyActor` _output))))
    (bind _keys (`BlueprintMapLibrary.Map_Keys` (`/Game/InventorySTM/Blueprints/SaveLoad/BP_SG_Level.ActorsAdded` (`self.As BP SG Level`))))
    (for _array_element_2 _keys
      (bind _returnvalue_4 (`GameplayStatics.GetActorOfClass` "/Game/InventorySTM/Blueprints/Containers/BP_Chest.BP_Chest_C"))
      (bind _output_2 (`|ConvertAsset` _array_element_2))
      (if (not (== _output_2 (`GameplayStatics.GetObjectClass` _returnvalue_4)))
        (`|SpawnActorFromClass` _output_2 (`BlueprintMapLibrary.Map_Find` (`/Game/InventorySTM/Blueprints/SaveLoad/BP_SG_Level.ActorsAdded` (`self.As BP SG Level`)) _array_element_2) "AlwaysSpawn" "OverrideRootScale" null null)))
    (else
      (bind _returnvalue_5 (`GameplayStatics.CreateSaveGameObject` "/Game/InventorySTM/Blueprints/SaveLoad/BP_SG_Level.BP_SG_Level_C"))
      (bind _output_get_3 (set `self.As BP SG Level` _returnvalue_5))
      (`GameplayStatics.SaveGameToSlot` _output_get_3 (`self.Level Data Slot`)))))

(event `self.ReceiveEndPlay`
  (params (EndPlayReason :type "EEndPlayReason Enum" :default "Destroyed"))
  (`GameplayStatics.SaveGameToSlot` (`self.As BP SG Level`) (`self.Level Data Slot`)))

(fn `UserConstructionScript`)