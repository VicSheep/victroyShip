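; Inventory component for players and containers such as chests, holding slot stacks with sizes and item classes from DT_ItemData.
; A per-tick sphere trace shows look-at prompts and feeds E-key interaction via a server event.
; Slot functions add, stack, swap, merge and drop items, with server wrappers and multicast updates.
; Updates trigger autosave: the player's contents go to the player save slot, others into the level save's container map, reloaded on BeginPlay.
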(event `self.ReceiveBeginPlay`
  (`KismetSystemLibrary.Delay` 0.2)
  (`self.Load Inventory`) ; Load Inventory Saved before "Resize"
  ;[0 0 0 0] Resize the array of items and create the message widget by adding it to the screen.
  (`KismetArrayLibrary.Array_Resize` (`self.Inventory Content`) (`self.Inventory Size`))
  (bind _returnvalue (`|CreateWidget` "/Game/InventorySTM/UI/Message/WBP_DisplayMessage.WBP_DisplayMessage_C"))
  (bind _output_get (set `self.Display Message` _returnvalue))
  (`UserWidget.AddToViewport` _output_get 0) ; If it is a solo game and you are NEVER going to migrate to multiplayer, you \ncan use the "Add To Viewport" node.
  ;[0 0 0 0] Auto Save
  (add `self.On Inventory Update` (delegate `Auto Save Inventory`)))

(event `Auto Save Inventory`
  ;[0 0 0 0] Auto Save
  (`self.Save Inventory`))

(event `self.ReceiveTick`
  (params (DeltaSeconds :type "Float (single-precision)"))
  ;[0 0 0 0] Interaction trace on tick
  (`self.Interaction Trace` (`self.Interaction Sphere Debug`)))

(event `Server Interact`
  (params (Target :type "Actor Object Reference"))
  (bind _returnvalue (`Actor.GetComponentByClass` Target "/Game/InventorySTM/Blueprints/Components/BPC_ItemData.BPC_ItemData_C"))
  (bind _asbp_ch_pawn (cast `/Game/InventorySTM/Core/BP_CH_Pawn` (`self.GetOwner`) :!pure true))
  ;[0.03125 0.03125 0.03125 0] Interact In Server & Owning Client
  (`/Engine/EditorBlueprintResources/StandardMacros.IsValid` _returnvalue
    (:`Is Valid`
      (message `/Game/InventorySTM/Interfaces/BPI_Interact.InteractWith` _returnvalue (cast `/Game/InventorySTM/Core/BP_CH_Pawn` (`self.GetOwner`) :!pure true)))
    (:`Is Not Valid`
      (`Actor.SetOwner` Target (`Pawn.GetController` _asbp_ch_pawn))
      (`self.On Local Interact` Target _asbp_ch_pawn))))

(event `On Local Interact`
  (params (`Target Actor` :type "Actor Object Reference") (Interactor :type "Actor Object Reference"))
  ;[0.03125 0.03125 0.03125 0] Interact In Server & Owning Client
  (message `/Game/InventorySTM/Interfaces/BPI_Interact.InteractWith` `Target Actor` (cast `/Game/InventorySTM/Core/BP_CH_Pawn` Interactor :!pure true)))

(event `MC_Update`
  ;[0 0 0 0] Multicast
  (`self.On Inventory Update`))

(event `SV Transfer Slots`
  (params (`Source Index` :type Integer) (`Source Inventory` :type "/Game/InventorySTM/Blueprints/Components/BPC_InventorySTM Object Reference") (`Destination Index` :type Integer))
  ;[0 0 0 0] Tranfer Slots In Inventory
  (`self.Transfer Slots` `Source Index` `Source Inventory` `Destination Index`))

(event `SV Remove From Inventory`
  (params (Index :type Integer) (`Remove Whole Stack` :type Boolean) (Consume :type Boolean))
  ;[0 0 0 0] Remove Slots From Inventory
  (`self.Remove From Inventory` Index `Remove Whole Stack` Consume))

(event `SV Drop Item`
  (params (`Item ID` :type Name) (Quantity :type Integer))
  ;[0 0 0 0] Drop Item
  (for _ (range Quantity)
    (`|SpawnActorFromClass` (`.ItemClass_10_467091E84048B55B5F8D1DA311E72611` (break `/Game/InventorySTM/Data/S_ItemStruct` (`self.Get Item Data` `Item ID`))) (`KismetMathLibrary.MakeTransform` (`self.Get Drop Location`)) "Undefined" "OverrideRootScale" null null)))

(event `Key|One`
  (params (Key :type "Key Structure"))
  ;[0.03125 0.03125 0.03125 0] Debug | Print Inventory Content
  (:`Pressed`
    (`self.Print Contents`)))

(event `Key|E`
  (params (Key :type "Key Structure"))
  ;[0.03125 0.03125 0.03125 0] Interact
  (:`Pressed`
    (bind _look_at_actor (`self.Look At Actor`)
      (:`then`
        (`self.Server Interact` _look_at_actor))
      (:`else`))))

(fn `Add To Inventory`
  (params (`Item ID` :type Name) (Quantity :type Integer))
  (returns (Success :type Boolean) (`Quantity Remaining` :type Integer))
  (locals (`Local Quantity Remaining` :type Integer) (`Local Has Failed` :type Boolean))
  (set `local.Local Quantity Remaining` Quantity)
  (while (and (> (`local.Local Quantity Remaining`) 0) (not (`local.Local Has Failed`)))
    (bind (_index _found_slot) (`self.Find Slot` (`local.Item ID`)))
    (if _found_slot
      (`self.Add To Stack` _index (`local.Quantity`))
      (`/Engine/EditorBlueprintResources/StandardMacros.DecrementInt` (`local.Local Quantity Remaining`))
      (elif (`self.Any Empty Slots Available?`)
        (bind _success (`self.Create New Stack` (`local.Item ID`) 1))
        (if _success
          (`/Engine/EditorBlueprintResources/StandardMacros.DecrementInt` (`local.Local Quantity Remaining`))
          (else
            (set `local.Local Has Failed` true)))
        (else
          (set `local.Local Has Failed` true)))))
  (`self.On Inventory Update`)
  (return (not (`local.Local Has Failed`)) (`local.Local Quantity Remaining`)))

(fn `Add To Stack`
  (params (Index :type Integer) (Quantity :type Integer))
  (bind (_output_itemid _output_quantity) (break `/Game/InventorySTM/Data/S_SlotStruct` (`|GetArrayItem` (`self.Inventory Content`) Index)))
  (`KismetArrayLibrary.Array_Set` (`self.Inventory Content`) Index (make `/Game/InventorySTM/Data/S_SlotStruct` _output_itemid (+ _output_quantity Quantity))))

(fn `Any Empty Slots Available?`
  (returns (`Has Empty Slot` :type Boolean) (`Empty Index` :type Integer))
  (for (_array_element _array_index) (`self.Inventory Content`)
    (if (== (`.Quantity_5_8A0477A246D6973817716C88C899E84B` (break `/Game/InventorySTM/Data/S_SlotStruct` _array_element)) 0)
      (return true _array_index)))
  (return false -1))

(fn `Create New Stack`
  (params (`Item ID` :type Name) (Quantity :type Integer))
  (returns (Success :type Boolean))
  (bind (_has_empty_slot _empty_index) (`self.Any Empty Slots Available?`))
  (if _has_empty_slot
    (`KismetArrayLibrary.Array_Set` (`self.Inventory Content`) _empty_index (make `/Game/InventorySTM/Data/S_SlotStruct` (`local.Item ID`) (`local.Quantity`)))
    (return true)))

(fn `Find Slot`
  (params (`Item ID` :type Name))
  (returns (Index :type Integer) (`Found Slot` :type Boolean))
  (for (_array_element _array_index) (`self.Inventory Content`)
    (bind (_itemid _quantity) (break `/Game/InventorySTM/Data/S_SlotStruct` _array_element))
    (if (== _itemid (`local.Item ID`))
      (if (< _quantity (`self.Get Max Stack Size` (`local.Item ID`)))
        (return _array_index true))))
  (return -1 false))

(fn `Get Drop Location`
  (returns (Location :type "Vector Structure"))
  (return (`Actor.K2_GetActorLocation` (`self.GetOwner`))))

(fn `Get Item Data`
  (params (`Item ID` :type Name))
  (returns (Data :type "/Game/InventorySTM/Data/S_ItemStruct Structure"))
  (bind _returnvalue (`|GetDataTableRow` "/Game/InventorySTM/Data/DT_ItemData.DT_ItemData" `Item ID`)
    (:`then`
      (return _returnvalue))))

(fn `Get Max Stack Size`
  (params (`Item ID` :type Name))
  (returns (StackSize :type Integer))
  (bind _returnvalue (`|GetDataTableRow` "/Game/InventorySTM/Data/DT_ItemData.DT_ItemData" `Item ID`)
    (:`then`
      (return (`.StackSize_13_0B6F248346F2269358FEF9AE4A9A0E19` (break `/Game/InventorySTM/Data/S_ItemStruct` _returnvalue))))
    (:`RowNotFound`
      (return -1) ; Invalid Value
    )))

(fn `GetPlayerPawn`
  (returns (`As BP CH Pawn` :type "/Game/InventorySTM/Core/BP_CH_Pawn Object Reference"))
  (`self.As BP CH Pawn`
    (:`then`
      _)
    (:`else`
      (bind _asbp_ch_pawn (cast `/Game/InventorySTM/Core/BP_CH_Pawn` (`GameplayStatics.GetPlayerPawn` 0)))
      (set `self.As BP CH Pawn` _asbp_ch_pawn)))
  (return (`self.As BP CH Pawn`)))

(fn `Interaction Trace`
  (params (DrawDebugType :type "EDrawDebugTrace Enum" :default "None"))
  (bind _returnvalue (`self.GetOwner`))
  (bind _returnvalue_2 (`Actor.K2_GetActorLocation` _returnvalue))
  (bind (_outhit _returnvalue_3) (`KismetSystemLibrary.SphereTraceSingle` _returnvalue_2 _returnvalue_2 100.0 "TraceTypeQuery1" false (`|MakeArray` _returnvalue) DrawDebugType true (struct :`R` 1.0 :`A` 1.0) (struct :`G` 1.0 :`A` 1.0) 0.1))
  (bind _output_get (set `self.Hit Struct |` _outhit))
  (set `self.Hit Actor` (`.HitActor` (`GameplayStatics.BreakHitResult` _output_get)))
  (if _returnvalue_3
    (bind _asbp_chest (cast `/Game/InventorySTM/Blueprints/Containers/BP_Chest` (`self.Hit Actor`))
      (:`then`
        (set `self.Look At Actor` null)
        (`/Game/InventorySTM/UI/Message/WBP_DisplayMessage.Show Message` (`self.Display Message`) "Open Chest")
        (set `/Game/InventorySTM/Core/BP_CH_Pawn.ChestToOpen` _asbp_chest (`self.GetPlayerPawn`)))
      (:`CastFailed`
        (set `/Game/InventorySTM/Core/BP_CH_Pawn.ChestToOpen` null (`self.GetPlayerPawn`))
        (if (!= (`self.Hit Actor`) (`self.Look At Actor`))
          (bind _output_get_2 (set `self.Look At Actor` (`self.Hit Actor`)))
          (bind _message (message `/Game/InventorySTM/Interfaces/BPI_Interact.LookAt` _output_get_2))
          (`/Game/InventorySTM/UI/Message/WBP_DisplayMessage.Show Message` (`self.Display Message`) _message))))
    (else
      (`/Engine/EditorBlueprintResources/StandardMacros.IsValid` (`self.Display Message`)
        (:`Is Valid`
          (set `self.Look At Actor` null)
          (`/Game/InventorySTM/UI/Message/WBP_DisplayMessage.Show Message` (`self.Display Message`) ""))))))

(fn `Load Inventory`
  (if (== (`self.GetOwner`) (`GameplayStatics.GetPlayerCharacter` 0))
    ;[0 0 0 0] Load Game for Player Data
    (bind _asbp_gi_main (cast `/Game/InventorySTM/Blueprints/SaveLoad/BP_GI_Main` (`GameplayStatics.GetGameInstance`)))
    (set `self.Inventory Content` (`/Game/InventorySTM/Blueprints/SaveLoad/BP_SG_Player.Inventory Content` (`/Game/InventorySTM/Blueprints/SaveLoad/BP_GI_Main.As BP SG Player` _asbp_gi_main)))
    (else
      (bind _asbp_gm_game (cast `/Game/InventorySTM/Core/BP_GM_Game` (`GameplayStatics.GetGameMode`)))
      (set `self.Inventory Content` (`.Contents_4_8DA494324A44606DC71EECAB7F75AB48` (break `/Game/InventorySTM/Data/S_ContainerStruct` (`BlueprintMapLibrary.Map_Find` (`/Game/InventorySTM/Blueprints/SaveLoad/BP_SG_Level.ContainersAdded` (`/Game/InventorySTM/Core/BP_GM_Game.As BP SG Level` _asbp_gm_game)) (`|ConvertAsset` self))))))))

(fn `Print Contents`
  (for (_array_element _array_index) (`self.Inventory Content`)
    (bind (_itemid _quantity) (break `/Game/InventorySTM/Data/S_SlotStruct` _array_element))
    (`KismetSystemLibrary.PrintString` (`KismetStringLibrary.Concat_StrStr` (`KismetStringLibrary.Conv_IntToString` _array_index) ":" (`KismetStringLibrary.Conv_NameToString` _itemid) "=" (`KismetStringLibrary.Conv_IntToString` _quantity)))))

(fn `Remove From Inventory`
  (params (Index :type Integer) (`Remove Whole Stack` :type Boolean) (`Is Consumed` :type Boolean))
  (locals (`Local Item` :type Name) (`Local Quantity` :type Integer))
  (bind (_output_itemid _output_quantity) (break `/Game/InventorySTM/Data/S_SlotStruct` (`|GetArrayItem` (`self.Inventory Content`) Index)))
  (bind (_itemid _quantity) (break `/Game/InventorySTM/Data/S_SlotStruct` (`|GetArrayItem` (`self.Inventory Content`) (`local.Index`))))
  (set `local.Local Item` _output_itemid)
  (set `local.Local Quantity` _output_quantity)
  (`|ExecutionSequence`
    (:`then_0`
      (if (or (`local.Remove Whole Stack`) (== (`local.Local Quantity`) 1))
        (`KismetArrayLibrary.Array_Set` (`self.Inventory Content`) (`local.Index`) (make `/Game/InventorySTM/Data/S_SlotStruct` "None"))
        (if (not (`local.Is Consumed`))
          (`self.SV Drop Item` (`local.Local Item`) (`local.Local Quantity`)))
        (else
          (`KismetArrayLibrary.Array_Set` (`self.Inventory Content`) (`local.Index`) (make `/Game/InventorySTM/Data/S_SlotStruct` _itemid (- _quantity 1)))
          (if (not (`local.Is Consumed`))
            (`self.SV Drop Item` (`local.Local Item`) 1)))))
    (:`then_1`
      (`self.MC_Update`))))

(fn `Save Inventory`
  (if (== (`self.GetOwner`) (`GameplayStatics.GetPlayerCharacter` 0))
    ;[0 0 0 0] Save Game For Player Data
    (bind _asbp_gi_main (cast `/Game/InventorySTM/Blueprints/SaveLoad/BP_GI_Main` (`GameplayStatics.GetGameInstance`)))
    (bind _as_bp_sg_player (`/Game/InventorySTM/Blueprints/SaveLoad/BP_GI_Main.As BP SG Player` _asbp_gi_main))
    (set `/Game/InventorySTM/Blueprints/SaveLoad/BP_SG_Player.Inventory Content` (`self.Inventory Content`) _as_bp_sg_player)
    (`GameplayStatics.SaveGameToSlot` _as_bp_sg_player "Data")
    (else
      (bind _asbp_gm_game (cast `/Game/InventorySTM/Core/BP_GM_Game` (`GameplayStatics.GetGameMode`)))
      (`BlueprintMapLibrary.Map_Add` (`/Game/InventorySTM/Blueprints/SaveLoad/BP_SG_Level.ContainersAdded` (`/Game/InventorySTM/Core/BP_GM_Game.As BP SG Level` _asbp_gm_game)) (`|ConvertAsset` self) (make `/Game/InventorySTM/Data/S_ContainerStruct` (`self.Inventory Content`))))))

(fn `Transfer Slots`
  (params (`Source Index` :type Integer) (`Source Inventory` :type "/Game/InventorySTM/Blueprints/Components/BPC_InventorySTM Object Reference") (`Destination Index` :type Integer))
  (locals (`Local Slot Content` :type "/Game/InventorySTM/Data/S_SlotStruct Structure"))
  (bind _local_slot_content_itemid (break `/Game/InventorySTM/Data/S_SlotStruct` (`local.Local Slot Content`)))
  (bind (_local_slot_content_itemid_2 _local_slot_content_quantity) (break `/Game/InventorySTM/Data/S_SlotStruct` (`local.Local Slot Content`)))
  (bind (_local_slot_content_itemid_3 _local_slot_content_quantity_2) (break `/Game/InventorySTM/Data/S_SlotStruct` (`local.Local Slot Content`)))
  (bind _stacksize (`self.Get Max Stack Size` _local_slot_content_itemid_3))
  (bind (_output_itemid _output_quantity) (break `/Game/InventorySTM/Data/S_SlotStruct` (`|GetArrayItem` (`self.Inventory Content`) (`local.Destination Index`))))
  (bind (_output_itemid_2 _output_quantity_2) (break `/Game/InventorySTM/Data/S_SlotStruct` (`|GetArrayItem` (`self.Inventory Content`) (`local.Destination Index`))))
  (bind _returnvalue (`KismetMathLibrary.Clamp` (- (+ _local_slot_content_quantity_2 _output_quantity_2) _stacksize) 0 _stacksize))
  (set `local.Local Slot Content` (`|GetArrayItem` (`/Game/InventorySTM/Blueprints/Components/BPC_InventorySTM.Inventory Content` `Source Inventory`) `Source Index`))
  (if (< `Destination Index` 0)
    _
    (elif (== (`.ItemID_4_6C53946244414507F6CC6A88B2CD4871` (break `/Game/InventorySTM/Data/S_SlotStruct` (`local.Local Slot Content`))) (`.ItemID_4_6C53946244414507F6CC6A88B2CD4871` (break `/Game/InventorySTM/Data/S_SlotStruct` (`|GetArrayItem` (`self.Inventory Content`) (`local.Destination Index`)))))
      (`KismetArrayLibrary.Array_Set` (`/Game/InventorySTM/Blueprints/Components/BPC_InventorySTM.Inventory Content` (`local.Source Inventory`)) (`local.Source Index`) (make `/Game/InventorySTM/Data/S_SlotStruct` (select `bool` (> _returnvalue 0) :`true` _local_slot_content_itemid) _returnvalue))
      (`KismetArrayLibrary.Array_Set` (`self.Inventory Content`) (`local.Destination Index`) (make `/Game/InventorySTM/Data/S_SlotStruct` _local_slot_content_itemid (`KismetMathLibrary.Clamp` (+ _local_slot_content_quantity _output_quantity) 0 (`self.Get Max Stack Size` _local_slot_content_itemid_2))))
      (`self.MC_Update`)
      (`self.MC_Update` (`local.Source Inventory`))
      (else
        (`KismetArrayLibrary.Array_Set` (`/Game/InventorySTM/Blueprints/Components/BPC_InventorySTM.Inventory Content` (`local.Source Inventory`)) (`local.Source Index`) (`|GetArrayItem` (`self.Inventory Content`) (`local.Destination Index`)))
        (`KismetArrayLibrary.Array_Set` (`self.Inventory Content`) (`local.Destination Index`) (`local.Local Slot Content`))
        (`self.MC_Update`)
        (`self.MC_Update` (`local.Source Inventory`))))))