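; Actor component that turns its owner into an item pickup for the InventorySTM inventory system, holding an item ID and quantity.
; On begin play it enables replication on the owning actor.
; Interacting adds the item to the player character's inventory component and destroys the owner when the add succeeds.
; Its LookAt function returns an empty string.
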(event `self.ReceiveBeginPlay`
  (`Actor.SetReplicates` (`self.GetOwner`) true))

(event `/Game/InventorySTM/Interfaces/BPI_Interact.InteractWith`
  (params (`Player Character` :type "/Game/InventorySTM/Core/BP_CH_Pawn Object Reference"))
  (bind _bpc_inventorystm (`/Game/InventorySTM/Core/BP_CH_Pawn.BPC_InventorySTM` `Player Character`))
  (bind (_itemid_datatable _itemid_rowname) (break `DataTableRowHandle` (`self.ItemID`)))
  ;[0 0 0 0] Interact
  (`/Engine/EditorBlueprintResources/StandardMacros.IsValid` _bpc_inventorystm
    (:`Is Valid`
      (bind _success (`/Game/InventorySTM/Blueprints/Components/BPC_InventorySTM.Add To Inventory` _bpc_inventorystm _itemid_rowname (`self.Quantity`)))
      (if _success
        (`Actor.K2_DestroyActor` (`self.GetOwner`))))))

(fn `LookAt`
  (returns (Message :type Text))
  (return ""))