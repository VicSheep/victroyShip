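; BP_Item is an item actor in the inventory system that records its presence and removal in the level's save data.
; After a short delay that lets the level SaveGame load, BeginPlay adds its class and transform to ActorsAdded through BP_GM_Game and saves the slot.
; ActorsAdded is keyed by class rather than by instance.
; On Destroyed it adds itself uniquely to ActorsRemoved without saving the slot.
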(event `self.ReceiveBeginPlay`
  (`KismetSystemLibrary.Delay` 0.2) ; The delay is necessary so that the SG Level Data is loaded first, \notherwise it will give error, since it will try to get it when it is not \nyet created.
  (bind _asbp_gm_game (cast `/Game/InventorySTM/Core/BP_GM_Game` (`GameplayStatics.GetGameMode`)))
  (bind _as_bp_sg_level (`/Game/InventorySTM/Core/BP_GM_Game.As BP SG Level` _asbp_gm_game))
  (`BlueprintMapLibrary.Map_Add` (`/Game/InventorySTM/Blueprints/SaveLoad/BP_SG_Level.ActorsAdded` _as_bp_sg_level) (`|ConvertAsset` (`GameplayStatics.GetObjectClass` self)) (`self.GetTransform`))
  (`GameplayStatics.SaveGameToSlot` _as_bp_sg_level (`/Game/InventorySTM/Core/BP_GM_Game.Level Data Slot` _asbp_gm_game)))

(event `self.ReceiveDestroyed`
  (bind _asbp_gm_game (cast `/Game/InventorySTM/Core/BP_GM_Game` (`GameplayStatics.GetGameMode`)))
  (`KismetArrayLibrary.Array_AddUnique` (`/Game/InventorySTM/Blueprints/SaveLoad/BP_SG_Level.ActorsRemoved` (`/Game/InventorySTM/Core/BP_GM_Game.As BP SG Level` _asbp_gm_game)) (`|ConvertAsset` self)))

(fn `UserConstructionScript`)