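; Player controller for an inventory system that handles item use, fast-slot hotkeys, interaction with chests and traders, fireball casting and pawn death.
; It creates the main widget for the local player and runs a timed trace for the interact prompt.
; Interface events forward storage, drop and busy-state changes to server events.
; Pawn damage feeds the health component, and death drops all items and removes the UI.
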(event `self.ReceivePossess`
  (params (PossessedPawn :type "Pawn Object Reference"))
  ;[0 0.04334 1] On Possess
  ;[0 0.1326 1] INIT
  (`/Engine/EditorBlueprintResources/ActorMacros.Switch Has Authority`
    (:`Authority`
      (`self.-Init`)
      (`self.-BindEvents`)
      (if (`KismetSystemLibrary.IsStandalone`)
        (if (`self.IsLocalPlayerController`) :!label _label
          (`/Engine/EditorBlueprintResources/StandardMacros.DoOnce` false
            (:`Completed`
              (bind _returnvalue (`|CreateWidget` "/Game/InventorySystem/Blueprints/UI/W_MainWidget.W_MainWidget_C" null self))
              (bind _output_get (set `self.MainWidget` _returnvalue))
              (`UserWidget.AddToViewport` _output_get 0)
              (`KismetSystemLibrary.K2_SetTimer` null "-InfoTrace" 0.25 true))))))))

(event `Key|LeftControl`
  (params (Key :type "Key Structure"))
  ;[0 1 0 1 110] KEYS, YOU CAN REPLACE THEM WITH YOUR INPUT BUTTONS IN PROJECT SETTINGS
  ;;[0 1 0] Left Ctrl
  (:`Pressed`
    (set `self.CtrlPressed` true))
  (:`Released`
    (set `self.CtrlPressed` false)))

(event `Key|LeftShift`
  (params (Key :type "Key Structure"))
  ;[0 1 0 1 110] KEYS, YOU CAN REPLACE THEM WITH YOUR INPUT BUTTONS IN PROJECT SETTINGS
  ;;[0 1 0] Left Shift
  (:`Pressed`
    (set `self.ShiftPressed` true))
  (:`Released`
    (set `self.ShiftPressed` false)))

(event `self.ReceiveBeginPlay`
  ;[0 0.05955 1] BEGIN PLAY
  ;[0 0.1326 1] INIT
  (`/Engine/EditorBlueprintResources/ActorMacros.Switch Has Authority`
    (:`Remote`
      (`KismetSystemLibrary.Delay` 1.0)
      (goto _label))))

(event `Key|Six`
  (params (Key :type "Key Structure"))
  ;[0 1 0 1 110] KEYS, YOU CAN REPLACE THEM WITH YOUR INPUT BUTTONS IN PROJECT SETTINGS
  ;;[0 1 0] Fast Panel Slots
  (:`Pressed`
    (bind _mainwidget (`self.MainWidget`)
      (:`then`
        (`/Game/InventorySystem/Blueprints/UI/FastPanel/W_FastPanel.-UseItemInSlot` (`/Game/InventorySystem/Blueprints/UI/W_MainWidget.W_FastPanel` _mainwidget) 5))
      (:`else`))))

(event `Key|One`
  (params (Key :type "Key Structure"))
  ;[0 1 0 1 110] KEYS, YOU CAN REPLACE THEM WITH YOUR INPUT BUTTONS IN PROJECT SETTINGS
  ;;[0 1 0] Fast Panel Slots
  (:`Pressed`
    (bind _mainwidget (`self.MainWidget`)
      (:`then`
        (`/Game/InventorySystem/Blueprints/UI/FastPanel/W_FastPanel.-UseItemInSlot` (`/Game/InventorySystem/Blueprints/UI/W_MainWidget.W_FastPanel` _mainwidget) 0))
      (:`else`))))

(event `Key|E`
  (params (Key :type "Key Structure"))
  ;[0 1 0 1 110] KEYS, YOU CAN REPLACE THEM WITH YOUR INPUT BUTTONS IN PROJECT SETTINGS
  ;;[0 1 0] E - Interact
  (:`Pressed`
    (`self.-InteractEvent`)))

(event `Key|Two`
  (params (Key :type "Key Structure"))
  ;[0 1 0 1 110] KEYS, YOU CAN REPLACE THEM WITH YOUR INPUT BUTTONS IN PROJECT SETTINGS
  ;;[0 1 0] Fast Panel Slots
  (:`Pressed`
    (bind _mainwidget (`self.MainWidget`)
      (:`then`
        (`/Game/InventorySystem/Blueprints/UI/FastPanel/W_FastPanel.-UseItemInSlot` (`/Game/InventorySystem/Blueprints/UI/W_MainWidget.W_FastPanel` _mainwidget) 1))
      (:`else`))))

(event `Key|Seven`
  (params (Key :type "Key Structure"))
  ;[0 1 0 1 110] KEYS, YOU CAN REPLACE THEM WITH YOUR INPUT BUTTONS IN PROJECT SETTINGS
  ;;[0 1 0] Fast Panel Slots
  (:`Pressed`
    (bind _mainwidget (`self.MainWidget`)
      (:`then`
        (`/Game/InventorySystem/Blueprints/UI/FastPanel/W_FastPanel.-UseItemInSlot` (`/Game/InventorySystem/Blueprints/UI/W_MainWidget.W_FastPanel` _mainwidget) 6))
      (:`else`))))

(event `-InteractEvent`
  (bind (_outlocation _outrotation) (`self.GetActorEyesViewPoint` (`self.K2_GetPawn`)))
  ;[0 1 0 1 110] KEYS, YOU CAN REPLACE THEM WITH YOUR INPUT BUTTONS IN PROJECT SETTINGS
  ;;[0 1 0] E - Interact
  (`/Engine/EditorBlueprintResources/ActorMacros.Switch Has Authority`
    (:`Authority`
      (bind _outhit (`KismetSystemLibrary.LineTraceSingle` _outlocation (+ (* (`KismetMathLibrary.GetForwardVector` _outrotation) 200.0) _outlocation) "TraceTypeQuery1"))
      (bind (_bblockinghit _binitialoverlap _time _distance _location _impactpoint _normal _impactnormal _physmat _hitactor) (`GameplayStatics.BreakHitResult` _outhit))
      (if _bblockinghit
        (bind (_success _actorref _busy) (message `/Game/InventorySystem/Blueprints/Data/Interfaces/BPI_Interact.-GetInfoToInteract` _hitactor))
        (if _success
          (message `/Game/InventorySystem/Blueprints/Data/Interfaces/BPI_Interact.-Interact` _hitactor self)
          (if (not _busy)
            (message `/Game/InventorySystem/Blueprints/Data/Interfaces/BPI_Interact.-OpenCloseInventory_Interface` self false)))))))

(event `/Game/InventorySystem/Blueprints/Data/Interfaces/BPI_Interact.-ItemUse`
  (params (ItemInfo :type "/Game/InventorySystem/Blueprints/Data/Structures/Str_ItemInfo Structure"))
  (bind _returnvalue (`self.K2_GetPawn`))
  (bind _returnvalue_2 (`self.GetComponentByClass` _returnvalue "/Game/InventorySystem/Blueprints/Components/BP_Health_Component.BP_Health_Component_C"))
  ;[0 0.3943 1] Use Item
  (`/Engine/EditorBlueprintResources/StandardMacros.IsValid` _returnvalue
    (:`Is Valid`
      (`/Engine/EditorBlueprintResources/StandardMacros.IsValid` _returnvalue_2
        (:`Is Valid`
          (`/Game/InventorySystem/Blueprints/Components/BP_Health_Component.-UpdateStats` _returnvalue_2 (`.ItemStats_30_21426AAE4C762987EB31F083701225CC` (break `/Game/InventorySystem/Blueprints/Data/Structures/Str_ItemInfo` ItemInfo))))))))

(event `Key|Three`
  (params (Key :type "Key Structure"))
  ;[0 1 0 1 110] KEYS, YOU CAN REPLACE THEM WITH YOUR INPUT BUTTONS IN PROJECT SETTINGS
  ;;[0 1 0] Fast Panel Slots
  (:`Pressed`
    (bind _mainwidget (`self.MainWidget`)
      (:`then`
        (`/Game/InventorySystem/Blueprints/UI/FastPanel/W_FastPanel.-UseItemInSlot` (`/Game/InventorySystem/Blueprints/UI/W_MainWidget.W_FastPanel` _mainwidget) 2))
      (:`else`))))

(event `Key|Eight`
  (params (Key :type "Key Structure"))
  ;[0 1 0 1 110] KEYS, YOU CAN REPLACE THEM WITH YOUR INPUT BUTTONS IN PROJECT SETTINGS
  ;;[0 1 0] Fast Panel Slots
  (:`Pressed`
    (bind _mainwidget (`self.MainWidget`)
      (:`then`
        (`/Game/InventorySystem/Blueprints/UI/FastPanel/W_FastPanel.-UseItemInSlot` (`/Game/InventorySystem/Blueprints/UI/W_MainWidget.W_FastPanel` _mainwidget) 7))
      (:`else`))))

(event `Key|Four`
  (params (Key :type "Key Structure"))
  ;[0 1 0 1 110] KEYS, YOU CAN REPLACE THEM WITH YOUR INPUT BUTTONS IN PROJECT SETTINGS
  ;;[0 1 0] Fast Panel Slots
  (:`Pressed`
    (bind _mainwidget (`self.MainWidget`)
      (:`then`
        (`/Game/InventorySystem/Blueprints/UI/FastPanel/W_FastPanel.-UseItemInSlot` (`/Game/InventorySystem/Blueprints/UI/W_MainWidget.W_FastPanel` _mainwidget) 3))
      (:`else`))))

(event `Key|Nine`
  (params (Key :type "Key Structure"))
  ;[0 1 0 1 110] KEYS, YOU CAN REPLACE THEM WITH YOUR INPUT BUTTONS IN PROJECT SETTINGS
  ;;[0 1 0] Fast Panel Slots
  (:`Pressed`
    (bind _mainwidget (`self.MainWidget`)
      (:`then`
        (`/Game/InventorySystem/Blueprints/UI/FastPanel/W_FastPanel.-UseItemInSlot` (`/Game/InventorySystem/Blueprints/UI/W_MainWidget.W_FastPanel` _mainwidget) 8))
      (:`else`))))

(event `Key|Five`
  (params (Key :type "Key Structure"))
  ;[0 1 0 1 110] KEYS, YOU CAN REPLACE THEM WITH YOUR INPUT BUTTONS IN PROJECT SETTINGS
  ;;[0 1 0] Fast Panel Slots
  (:`Pressed`
    (bind _mainwidget (`self.MainWidget`)
      (:`then`
        (`/Game/InventorySystem/Blueprints/UI/FastPanel/W_FastPanel.-UseItemInSlot` (`/Game/InventorySystem/Blueprints/UI/W_MainWidget.W_FastPanel` _mainwidget) 4))
      (:`else`))))

(event `Key|Zero`
  (params (Key :type "Key Structure"))
  ;[0 1 0 1 110] KEYS, YOU CAN REPLACE THEM WITH YOUR INPUT BUTTONS IN PROJECT SETTINGS
  ;;[0 1 0] Fast Panel Slots
  (:`Pressed`
    (bind _mainwidget (`self.MainWidget`)
      (:`then`
        (`/Game/InventorySystem/Blueprints/UI/FastPanel/W_FastPanel.-UseItemInSlot` (`/Game/InventorySystem/Blueprints/UI/W_MainWidget.W_FastPanel` _mainwidget) 9))
      (:`else`))))

(event `/Game/InventorySystem/Blueprints/Data/Interfaces/BPI_Interact.-OpenCloseInventory_Interface`
  (params (Close :type Boolean))
  ;[1 1 1] Open Close Interface
  (`self.-OpenCloseInv_Server` Close))

(event `AnyDamage_ControlledPawn`
  (params (DamagedActor :type "Actor Object Reference") (Damage :type "Float (double-precision)") (DamageType :type "DamageType Object Reference") (InstigatedBy :type "Controller Object Reference") (DamageCauser :type "Actor Object Reference"))
  (bind _returnvalue (`self.K2_GetPawn`))
  (bind _returnvalue_2 (`self.GetComponentByClass` _returnvalue "/Game/InventorySystem/Blueprints/Components/BP_Health_Component.BP_Health_Component_C"))
  ;[1 1 1] Any Damage
  (`/Engine/EditorBlueprintResources/StandardMacros.IsValid` _returnvalue
    (:`Is Valid`
      (`/Engine/EditorBlueprintResources/StandardMacros.IsValid` _returnvalue_2
        (:`Is Valid`
          (`/Game/InventorySystem/Blueprints/Components/BP_Health_Component.-UpdateHealth` _returnvalue_2 (`KismetMathLibrary.Conv_IntToDouble` (* (`.ReturnValue` (`KismetMathLibrary.FMod` Damage 1.0)) -1))))))))

(event `-OpenCloseInv_Server`
  (params (Close :type Boolean))
  ;[1 1 1] Open Close Interface
  (if Close
    (if (`self.InventoryOpened`)
      (`self.-OpenCloseInventory`))
    (elif (not (`self.InventoryOpened`))
      (`self.-OpenCloseInventory`))))

(event `Key|I`
  (params (Key :type "Key Structure"))
  ;[0 1 0 1 110] KEYS, YOU CAN REPLACE THEM WITH YOUR INPUT BUTTONS IN PROJECT SETTINGS
  ;;[0 1 0] I - Inventory
  (:`Pressed`
    (`self.-OpenCloseInventory`)))

(event `-DropAllItemsToWorld`
  ;[1 1 1] Drop All items to World
  (`/Game/InventorySystem/Blueprints/Components/BP_Storage_Component.-DropAllItemsToWorld` (`self.BP_Storage_Component`)))

(event `/Game/InventorySystem/Blueprints/Data/Interfaces/BPI_Interact.-AddItemToTargetStorage`
  (params (TargetStorage :type "/Game/InventorySystem/Blueprints/Components/BP_Storage_Component Object Reference") (Item :type "Array of /Game/InventorySystem/Blueprints/Data/Structures/Str_Item Structure (by ref)"))
  ;[1 1 1] Add Item to target Storage
  (for _array_element Item
    (bind (_itemclass _amount) (break `/Game/InventorySystem/Blueprints/Data/Structures/Str_Item` _array_element))
    (`self.-AddItemToStorage_Server` TargetStorage _itemclass _amount true)))

(event `-OpenCloseInventory`
  (bind _returnvalue (`GameplayStatics.GetPlayerController` 0))
  ;[0 1 0 1 110] KEYS, YOU CAN REPLACE THEM WITH YOUR INPUT BUTTONS IN PROJECT SETTINGS
  ;;[0 1 0] I - Inventory
  (bind _mainwidget (`self.MainWidget`)
    (:`then`
      (`/Engine/EditorBlueprintResources/StandardMacros.IsValid` (`self.GetComponentByClass` "/Game/InventorySystem/Blueprints/Components/BP_Storage_Component.BP_Storage_Component_C")
        (:`Is Valid`
          (bind _w_inventory (`/Game/InventorySystem/Blueprints/UI/W_MainWidget.W_Inventory` _mainwidget))
          (`/Game/InventorySystem/Blueprints/UI/Inventory/W_Inventory.-UpdateInventory` _w_inventory)
          (bind _returnvalue_2 (`Widget.IsVisible` _w_inventory))
          (`Widget.SetVisibility` _w_inventory (select `bool` _returnvalue_2 :`false` "Visible" :`true` "Hidden" :!type "ESlateVisibility Enum"))
          (`self.-SetInput_Server` _returnvalue_2)
          (`KismetSystemLibrary.Delay` (select `bool` (`KismetSystemLibrary.IsStandalone`) :`false` 0.1 :!type "Float (single-precision)"))
          (set `PlayerController.bShowMouseCursor` _returnvalue_2 _returnvalue)
          (if (`self.InventoryOpened`)
            (`WidgetBlueprintLibrary.SetInputMode_GameAndUIEx` _returnvalue null "LockInFullscreen" false)
            (else
              (`WidgetBlueprintLibrary.SetInputMode_GameOnly` _returnvalue)
              (`Widget.SetVisibility` (`/Game/InventorySystem/Blueprints/UI/W_MainWidget.W_DropCounter` _mainwidget) "Hidden"))))
        (:`Is Not Valid`
          (`Widget.SetVisibility` _w_inventory "Hidden")
          (`WidgetBlueprintLibrary.SetInputMode_GameOnly` (`GameplayStatics.GetPlayerController` 0)))))
    (:`else`)))

(event `/Game/InventorySystem/Blueprints/Data/Interfaces/BPI_Interact.-Chest_Interact_Reset`
  (params (Chest :type "/Game/InventorySystem/Blueprints/Chest/BP_Chest_Master Object Reference") (Busy :type Boolean))
  ;[1 1 1] Interface - Set Busy Chest
  (`/Engine/EditorBlueprintResources/StandardMacros.IsValid` Chest
    (:`Is Valid`
      (`self.-SetBusy_Chest_Server` Busy Chest))))

(event `/Game/InventorySystem/Blueprints/Data/Interfaces/BPI_Interact.-Trader_Interact_Reset`
  (params (Trader :type "/Game/InventorySystem/Blueprints/Trader/BP_Trader_Master Object Reference") (Busy :type Boolean))
  ;[1 1 1] Set Busy - Trader
  (`/Engine/EditorBlueprintResources/StandardMacros.IsValid` Trader
    (:`Is Valid`
      (`self.-SetBusy_Trader_Server` Busy Trader))))

(event `/Game/InventorySystem/Blueprints/Data/Interfaces/BPI_Interact.-SetStorageItem`
  (params (TargetStorage :type "/Game/InventorySystem/Blueprints/Components/BP_Storage_Component Object Reference") (Index :type Integer) (ItemClass :type "/Game/InventorySystem/Blueprints/Items/BP_Items_Master Class Reference") (Amount :type Integer))
  ;[1 1 1] Set Storage Item
  (`self.-SetStorageItem_Server` TargetStorage Index ItemClass Amount))

(event `-SetInput_Server`
  (params (InventoryOpened :type Boolean))
  ;[0 1 0 1 110] KEYS, YOU CAN REPLACE THEM WITH YOUR INPUT BUTTONS IN PROJECT SETTINGS
  ;;[0 1 0] I - Inventory
  (set `self.InventoryOpened` InventoryOpened))

(event `-SetBusy_Trader_Server`
  (params (Busy :type Boolean) (Target :type "/Game/InventorySystem/Blueprints/Trader/BP_Trader_Master Object Reference"))
  ;[1 1 1] Set Busy - Trader
  (set `/Game/InventorySystem/Blueprints/Trader/BP_Trader_Master.Busy` Busy Target))

(event `-SetBusy_Chest_Server`
  (params (Busy :type Boolean) (Target :type "/Game/InventorySystem/Blueprints/Chest/BP_Chest_Master Object Reference"))
  ;[1 1 1] Interface - Set Busy Chest
  (set `/Game/InventorySystem/Blueprints/Chest/BP_Chest_Master.Busy` Busy Target))

(event `-SetStorageItem_Server`
  (params (Target :type "/Game/InventorySystem/Blueprints/Components/BP_Storage_Component Object Reference") (Index :type Integer) (ItemClass :type "/Game/InventorySystem/Blueprints/Items/BP_Items_Master Class Reference") (Amount :type Integer))
  ;[1 1 1] Set Storage Item
  (`KismetArrayLibrary.Array_Set` (`/Game/InventorySystem/Blueprints/Components/BP_Storage_Component.Storage` Target) Index (make `/Game/InventorySystem/Blueprints/Data/Structures/Str_Item` ItemClass Amount)))

(event `Key|LeftMouseButton`
  (params (Key :type "Key Structure"))
  ;[0 1 0 1 110] KEYS, YOU CAN REPLACE THEM WITH YOUR INPUT BUTTONS IN PROJECT SETTINGS
  ;;[0 1 0] Spawn Fireball
  (:`Pressed`
    (bind _returnvalue (`self.-CheckWidgetsForOpen`))
    (if (and (not _returnvalue) (not (`self.IsDead`)))
      (`self.-SpawnFireBall`))))

(event `/Game/InventorySystem/Blueprints/Data/Interfaces/BPI_Interact.-DropItemToWorld`
  (params (TargetStorage :type "/Game/InventorySystem/Blueprints/Components/BP_Storage_Component Object Reference") (ItemClass :type "/Game/InventorySystem/Blueprints/Items/BP_Items_Master Class Reference") (Amount :type Integer) (Id :type Integer) (InventorySlot :type "/Game/InventorySystem/Blueprints/UI/Inventory/W_Inventory_Slot Object Reference"))
  ;[1 1 1] Drop Item To World
  (`self.-DropItemToWorld_Server` TargetStorage ItemClass Amount Id))

(event `/Game/InventorySystem/Blueprints/Data/Interfaces/BPI_Interact.-AddItemToStorageEvent`
  (params (TargetStorage :type "/Game/InventorySystem/Blueprints/Components/BP_Storage_Component Object Reference") (Item :type "/Game/InventorySystem/Blueprints/Items/BP_Items_Master Class Reference") (Amount :type Integer) (`UpdateInventory?` :type Boolean) (Index :type Integer))
  ;[1 1 1] Add Item To Storage
  (`self.-AddItemToStorage_Server` TargetStorage Item Amount `UpdateInventory?`))

(event `-SpawnFireBall`
  (bind _returnvalue (`self.GetComponentByClass` (`self.K2_GetPawn`) "/Game/InventorySystem/Blueprints/Components/BP_Health_Component.BP_Health_Component_C"))
  ;[0 1 0 1 110] KEYS, YOU CAN REPLACE THEM WITH YOUR INPUT BUTTONS IN PROJECT SETTINGS
  ;;[0 1 0] Spawn Fireball
  (if (>= (`/Game/InventorySystem/Blueprints/Components/BP_Health_Component.CurrentMP` _returnvalue) 5.0)
    (`|SpawnActorFromClass` "/Game/InventorySystem/Blueprints/BP_Fireball.BP_Fireball_C" (`KismetMathLibrary.MakeTransform` (`self.GetActorEyesViewPoint` (`self.K2_GetPawn`)) (`self.GetControlRotation`) (`KismetMathLibrary.Conv_DoubleToVector` 0.25)) "AlwaysSpawn" "OverrideRootScale" self (`self.K2_GetPawn` self))
    (`/Engine/EditorBlueprintResources/StandardMacros.IsValid` _returnvalue
      (:`Is Valid`
        (`/Game/InventorySystem/Blueprints/Components/BP_Health_Component.-UpdateMP` _returnvalue -5.0)))))

(event `-AddItemToStorage_Server`
  (params (Target :type "/Game/InventorySystem/Blueprints/Components/BP_Storage_Component Object Reference") (Item :type "/Game/InventorySystem/Blueprints/Items/BP_Items_Master Class Reference") (Amount :type Integer) (`UpdateInventory?` :type Boolean))
  ;[1 1 1] Add Item To Storage
  (`/Game/InventorySystem/Blueprints/Components/BP_Storage_Component.-AddItem` Target Item Amount `UpdateInventory?`))

(event `-DropItemToWorld_Server`
  (params (Target :type "/Game/InventorySystem/Blueprints/Components/BP_Storage_Component Object Reference") (ItemClass :type "/Game/InventorySystem/Blueprints/Items/BP_Items_Master Class Reference") (Amount :type Integer) (StorageId :type Integer))
  ;[1 1 1] Drop Item To World
  (bind _success (`/Game/InventorySystem/Blueprints/Components/BP_Storage_Component.-DropItemToWorld` Target ItemClass Amount StorageId))
  (if _success
    (`/Game/InventorySystem/Blueprints/Components/BP_Storage_Component.-UpdateInventoryWidget_Client` (`self.BP_Storage_Component`) (select `bool` (`KismetSystemLibrary.IsStandalone`) :`false` 0.1 :!type "Float (single-precision)"))))

(event `-ControlledPawnIsDead`
  ;[1 0 0] Controlled Pawn Is Dead
  (if (not (`self.IsDead`))
    (set `self.IsDead` true)
    (`|ExecutionSequence`
      (:`then_0`
        (`self.DisableInput` (`self.K2_GetPawn`) self)
        (`self.-DropAllItemsToWorld`)
        (message `/Game/InventorySystem/Blueprints/Data/Interfaces/BPI_Interact.-OpenCloseInventory_Interface` self true))
      (:`then_1`
        (`self.-DestroyMainWidget`)))))

(event `-DestroyMainWidget`
  ;[1 0 0] Controlled Pawn Is Dead
  (bind _mainwidget (`self.MainWidget`)
    (:`then`
      (`Widget.RemoveFromParent` _mainwidget))
    (:`else`)))

(fn `-AddItemToStorage`
  (params (TargetStorage :type "/Game/InventorySystem/Blueprints/Components/BP_Storage_Component Object Reference") (Item :type "/Game/InventorySystem/Blueprints/Items/BP_Items_Master Class Reference") (Amount :type Integer) (`UpdateInvetory?` :type Boolean))
  (returns (Success :type Boolean) (Index :type Integer) (Rest :type Integer) (AddedItems :type Integer))
  (bind _bp_storage_component (`self.BP_Storage_Component`))
  (bind (_success _index _rest _addeditems) (`/Game/InventorySystem/Blueprints/Components/BP_Storage_Component.-AddItem` _bp_storage_component Item Amount `UpdateInvetory?`))
  (if _success
    (`/Game/InventorySystem/Blueprints/Components/BP_Storage_Component.-UpdateInventoryWidget_Client` _bp_storage_component 0.1)
    (return _success _index _rest _addeditems)
    (else
      (return false _index _rest _addeditems))))

(fn `-BindEvents`
  (bind _returnvalue (`self.K2_GetPawn`))
  (bind _returnvalue_2 (`self.GetComponentByClass` _returnvalue "/Game/InventorySystem/Blueprints/Components/BP_Health_Component.BP_Health_Component_C"))
  (add `self.OnTakeAnyDamage` _returnvalue (`|CreateDelegate` :!event `AnyDamage_ControlledPawn`))
  (`/Engine/EditorBlueprintResources/StandardMacros.IsValid` _returnvalue_2
    (:`Is Valid`
      (add `/Game/InventorySystem/Blueprints/Components/BP_Health_Component.IsDeadDispatcher` _returnvalue_2 (`|CreateDelegate` :!event `-ControlledPawnIsDead`)))))

(fn `-CheckWidgetsForOpen`
  (returns (ReturnValue :type Boolean))
  (bind _mainwidget (`self.MainWidget`)
    (:`then`
      (return (or (`Widget.IsVisible` (`/Game/InventorySystem/Blueprints/UI/W_MainWidget.W_Chest` _mainwidget)) (`Widget.IsVisible` (`/Game/InventorySystem/Blueprints/UI/W_MainWidget.W_Inventory` _mainwidget)) (`Widget.IsVisible` (`/Game/InventorySystem/Blueprints/UI/W_MainWidget.W_Trader` _mainwidget)))))
    (:`else`
      (return false))))

(fn `-GetInfoToInteract`
  (returns (Success :type Boolean) (ActorRef :type "Actor Object Reference") (Busy :type Boolean))
  (return false null false))

(fn `-InfoTrace`
  (bind (_outlocation _outrotation) (`self.GetActorEyesViewPoint` (`self.K2_GetPawn`)))
  (bind _outhit (`KismetSystemLibrary.LineTraceSingle` _outlocation (+ (* (`KismetMathLibrary.GetForwardVector` _outrotation) 200.0) _outlocation) "TraceTypeQuery1"))
  (bind (_bblockinghit _binitialoverlap _time _distance _location _impactpoint _normal _impactnormal _physmat _hitactor) (`GameplayStatics.BreakHitResult` _outhit))
  (if _bblockinghit
    (bind (_success _actorref) (message `/Game/InventorySystem/Blueprints/Data/Interfaces/BPI_Interact.-GetInfoToInteract` _hitactor))
    (bind _asbp_chest_master (cast `/Game/InventorySystem/Blueprints/Chest/BP_Chest_Master` _actorref)
      (:`then`
        (if (`/Game/InventorySystem/Blueprints/Chest/BP_Chest_Master.Busy` _asbp_chest_master)
          (`/Game/InventorySystem/Blueprints/UI/W_PressE.-Update` (`/Game/InventorySystem/Blueprints/UI/W_MainWidget.W_PressE` (`self.MainWidget`)) false :!label _label)
          (else
            (if _success :!label _label_2
              (if (not (`Widget.IsVisible` (`/Game/InventorySystem/Blueprints/UI/W_MainWidget.W_PressE` (`self.MainWidget`))))
                (`/Game/InventorySystem/Blueprints/UI/W_PressE.-Update` (`/Game/InventorySystem/Blueprints/UI/W_MainWidget.W_PressE` (`self.MainWidget`)) true))
              (else
                (goto _label))))))
      (:`CastFailed`
        (bind _asbp_trader_master (cast `/Game/InventorySystem/Blueprints/Trader/BP_Trader_Master` _actorref)
          (:`then`
            (if (`/Game/InventorySystem/Blueprints/Trader/BP_Trader_Master.Busy` _asbp_trader_master)
              (goto _label)
              (else
                (goto _label_2))))
          (:`CastFailed`
            (goto _label_2)))))
    (else
      (`/Game/InventorySystem/Blueprints/UI/W_PressE.-Update` (`/Game/InventorySystem/Blueprints/UI/W_MainWidget.W_PressE` (`self.MainWidget`)) false))))

(fn `-Init`
  (`/Game/InventorySystem/Blueprints/Components/BP_Storage_Component.-Init` (`self.BP_Storage_Component`)))

(fn `-InteractWithRef`
  (returns (Success :type Boolean) (Pawn :type "Pawn Object Reference") (PlayerController :type "PlayerController Object Reference") (StorageRef :type "/Game/InventorySystem/Blueprints/Components/BP_Storage_Component Object Reference") (InventoryOpened :type Boolean) (ShiftPressed :type Boolean) (CtrlPressed :type Boolean) (IsDead :type Boolean) (MainWidget :type "/Game/InventorySystem/Blueprints/UI/W_MainWidget Object Reference"))
  (return true (`self.K2_GetPawn`) self (`self.BP_Storage_Component`) (`self.InventoryOpened`) (`self.ShiftPressed`) (`self.CtrlPressed`) (`self.IsDead`) (`self.MainWidget`)))

(fn `UserConstructionScript`)