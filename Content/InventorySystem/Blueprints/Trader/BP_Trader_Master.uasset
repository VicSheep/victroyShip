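; BP_Trader_Master is an interactable trader actor that shows its inventory in the interacting player's trader widget.
; BeginPlay initializes its storage component, delayed outside standalone play, and the construction script sets its text label.
; Interact opens the widget through a Multi event and marks the trader busy, letting only that same player trigger a close.
; Tick watches that player's distance, and moving out of range clears busy, saves slot positions and hides the widget.
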(event `-Close_Multi`
  (bind _playercontrollerinteract (`self.PlayerControllerInteract`))
  ;[1 1 1] Close Multi
  (bind (_success _pawn _playercontroller _storageref _inventoryopened _shiftpressed _ctrlpressed _isdead _mainwidget) (message `/Game/InventorySystem/Blueprints/Data/Interfaces/BPI_Interact.-InteractWithRef` _playercontrollerinteract))
  (`/Engine/EditorBlueprintResources/StandardMacros.IsValid` _mainwidget
    (:`Is Valid`
      (`/Game/InventorySystem/Blueprints/UI/Trader/W_Trader.-Close` (`/Game/InventorySystem/Blueprints/UI/W_MainWidget.W_Trader` _mainwidget))
      (message `/Game/InventorySystem/Blueprints/Data/Interfaces/BPI_Interact.-OpenCloseInventory_Interface` _playercontrollerinteract true))))

(event `self.ReceiveBeginPlay`
  ;[1 1 1] Begin Play
  (`KismetSystemLibrary.Delay` (select `bool` (`KismetSystemLibrary.IsStandalone`) :`false` 4.0 :!type "Float (single-precision)"))
  (`/Game/InventorySystem/Blueprints/Components/BP_Storage_Component.-Init` (`self.BP_Storage_Component`)))

(event `/Game/InventorySystem/Blueprints/Data/Interfaces/BPI_Interact.-Interact`
  (params (PlayerController :type "PlayerController Object Reference"))
  ;[1 1 1] Interact
  (if (not (`self.Busy`))
    (`self.-OpenChest` PlayerController)
    (else
      (bind _playercontrollerinteract (`self.PlayerControllerInteract`)
        (:`then`
          (if (== _playercontrollerinteract PlayerController)
            (`self.-Close_Multi`)))
        (:`else`)))))

(event `-OpenChest_Multi`
  (params (PlayerControllerInteract :type "PlayerController Object Reference"))
  ;[1 1 1] Open
  (set `self.PlayerControllerInteract` PlayerControllerInteract)
  (bind (_success _pawn _playercontroller _storageref _inventoryopened _shiftpressed _ctrlpressed _isdead _mainwidget) (message `/Game/InventorySystem/Blueprints/Data/Interfaces/BPI_Interact.-InteractWithRef` (`self.PlayerControllerInteract`)))
  (if (not (`KismetSystemLibrary.IsDedicatedServer`))
    (`/Engine/EditorBlueprintResources/StandardMacros.IsValid` _mainwidget
      (:`Is Valid`
        (bind _w_trader (`/Game/InventorySystem/Blueprints/UI/W_MainWidget.W_Trader` _mainwidget))
        (set `/Game/InventorySystem/Blueprints/UI/Trader/W_Trader.TraderRef` self _w_trader)
        (set `/Game/InventorySystem/Blueprints/UI/Trader/W_Trader.InteractOwnerController` (`self.PlayerControllerInteract`) _w_trader)
        (if (not (`Widget.IsVisible` _w_trader))
          (set `/Game/InventorySystem/Blueprints/UI/Trader/W_Trader.StorageComponentRef` (`self.BP_Storage_Component`) _w_trader)
          (`/Game/InventorySystem/Blueprints/UI/Trader/W_Trader.-UpdateStorageGrid` _w_trader (`/Game/InventorySystem/Blueprints/Components/BP_Storage_Component.SavedSlotsPositions` (`self.BP_Storage_Component`)))
          (`Widget.SetVisibility` _w_trader "Visible"))))))

(event `-OpenChest`
  (params (PlayerControllerInteract :type "PlayerController Object Reference"))
  ;[1 1 1] Open
  (set `self.Busy` true)
  (`self.-OpenChest_Multi` PlayerControllerInteract))

(event `self.ReceiveTick`
  (params (DeltaSeconds :type "Float (single-precision)"))
  ;[1 1 1] Distance to Close Trader Widget
  (bind _playercontrollerinteract (`self.PlayerControllerInteract`)
    (:`then`
      (if (>= (`self.GetDistanceTo` (`Controller.K2_GetPawn` _playercontrollerinteract)) 300.0)
        (set `self.Busy` false)
        (bind (_success _pawn _playercontroller _storageref _inventoryopened _shiftpressed _ctrlpressed _isdead _mainwidget) (message `/Game/InventorySystem/Blueprints/Data/Interfaces/BPI_Interact.-InteractWithRef` _playercontrollerinteract))
        (`/Engine/EditorBlueprintResources/StandardMacros.IsValid` _mainwidget
          (:`Is Valid`
            (bind _w_trader (`/Game/InventorySystem/Blueprints/UI/W_MainWidget.W_Trader` _mainwidget))
            (bind _savedpositionslots (`/Game/InventorySystem/Blueprints/UI/Trader/W_Trader.-SaveSlotsPositions` _w_trader))
            (set `/Game/InventorySystem/Blueprints/Components/BP_Storage_Component.SavedSlotsPositions` _savedpositionslots (`self.BP_Storage_Component`))
            (`Widget.SetVisibility` _w_trader "Hidden")
            (set `self.PlayerControllerInteract` null)))))
    (:`else`)))

(fn `-AddItemToStorage`
  (params (TargetStorage :type "/Game/InventorySystem/Blueprints/Components/BP_Storage_Component Object Reference") (Item :type "/Game/InventorySystem/Blueprints/Items/BP_Items_Master Class Reference") (Amount :type Integer) (`UpdateInvetory?` :type Boolean))
  (returns (Success :type Boolean) (Index :type Integer) (Rest :type Integer) (AddedItems :type Integer))
  (return false 0 0 0))

(fn `-GetInfoToInteract`
  (returns (Success :type Boolean) (ActorRef :type "Actor Object Reference") (Busy :type Boolean))
  (return true self (`self.Busy`)))

(fn `-InteractWithRef`
  (returns (Success :type Boolean) (Pawn :type "Pawn Object Reference") (PlayerController :type "PlayerController Object Reference") (StorageRef :type "/Game/InventorySystem/Blueprints/Components/BP_Storage_Component Object Reference") (InventoryOpened :type Boolean) (ShiftPressed :type Boolean) (CtrlPressed :type Boolean) (IsDead :type Boolean) (MainWidget :type "/Game/InventorySystem/Blueprints/UI/W_MainWidget Object Reference"))
  (return false null null null false false false false null))

(fn `UserConstructionScript`
  (`TextRenderComponent.K2_SetText` (`self.TextRender`) (`self.Text`)))