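; BP_Tree is a tree actor that catches fire the first time it takes damage.
; A Damaged flag ensures only the first AnyDamage event triggers the Fire event.
; Fire activates the PFire effect for a short delay, then switches it off and swaps the Sphere mesh material to black for a burnt look.
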(event `self.ReceiveAnyDamage`
  (params (Damage :type "Float (single-precision)") (DamageType :type "DamageType Object Reference") (InstigatedBy :type "Controller Object Reference") (DamageCauser :type "Actor Object Reference"))
  (if (not (`self.Damaged`))
    (set `self.Damaged` true)
    (`self.-Fire`)))

(event `-Fire`
  (`ActorComponent.SetActive` (`self.P_Fire`) true true)
  (`KismetSystemLibrary.Delay` 3.0)
  (`ActorComponent.SetActive` (`self.P_Fire`) false true)
  (`PrimitiveComponent.SetMaterial` (`self.Sphere`) 0 "/Game/InventorySystem/DemoContent/Materials/M_Black.M_Black"))

(fn `UserConstructionScript`)