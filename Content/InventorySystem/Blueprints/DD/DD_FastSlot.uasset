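; DD_FastSlot is the drag-and-drop operation for inventory fast slots, deciding how much of a stack is being dragged.
; On each Dragged event it reads modifier keys from the player controller: Ctrl takes one, Shift takes up to ten, otherwise the whole stack.
; A DoOnce, reset and re-entered through a Sequence, updates the source slot's displayed amount to the clamped remainder as a visual-only change.
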(event `self.Dragged`
  (params (PointerEvent :type "PointerEvent Structure (by ref)"))
  (bind _startamount (`self.StartAmount`))
  (bind (_success _pawn _playercontroller _storageref _inventoryopened _shiftpressed _ctrlpressed) (message `/Game/InventorySystem/Blueprints/Data/Interfaces/BPI_Interact.-InteractWithRef` (`self.PlayerController`)))
  (`|ExecutionSequence`
    (:`then_0`
      (if _ctrlpressed
        (set `self.Amount` 1)
        (goto _label :!via `Reset`)
        (elif _shiftpressed
          (set `self.Amount` (select `bool` (< _startamount 10) :`false` 10 :`true` _startamount))
          (goto _label :!via `Reset`)
          (else
            (set `self.Amount` (`self.StartAmount`))
            (goto _label :!via `Reset`)))))
    (:`then_1`
      (`/Engine/EditorBlueprintResources/StandardMacros.DoOnce` false :!label _label
        (:`Completed`
          (`/Game/InventorySystem/Blueprints/UI/FastPanel/W_FastPanel_Slot.-UpdateAmountOnlyVisual` (`self.DraggedSlot`) (`KismetMathLibrary.Max` (- (`self.StartAmount`) (`self.Amount`)))))))))