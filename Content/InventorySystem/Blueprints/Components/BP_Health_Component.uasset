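; Pawn component that tracks health, mana, hunger and thirst for the inventory system and applies item stat effects to them.
; Looping timers drain hunger and thirst, damaging health at zero, and regenerate mana until full, despite all three being named "Regeneration".
; Zero health sets the dead flag, clears the timers and fires the death dispatcher.
; RepNotifies on the four stats refresh the stats widget through the owner's controller.
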(event `-InitOwner`
  ;[1 1 1] Init
  (bind _aspawn (cast `Pawn` (`self.GetOwner`)))
  (set `self.Controller` (`Pawn.GetController` _aspawn))
  (`KismetSystemLibrary.Delay` (select `bool` (`KismetSystemLibrary.IsStandalone`) :`false` 3.0 :!type "Float (single-precision)"))
  (`self.-UpdateHealth` 0.0)
  (`|ExecutionSequence`
    (:`then_0`
      (if (`self.Hunger`)
        (bind _returnvalue (`KismetSystemLibrary.K2_SetTimer` null "-RegenerationHunger" (`self.HungerTimerForPoint`) true))
        (set `self.Timer-RegenerationHunger` _returnvalue)))
    (:`then_1`
      (if (`self.Thirst`)
        (bind _returnvalue_2 (`KismetSystemLibrary.K2_SetTimer` null "-RegenerationThirst" (`self.ThirstTimerForPoint`) true))
        (set `self.Timer-RegenerationThirst` _returnvalue_2)))))

(event `-UpdateHealth`
  (params (Health :type "Float (double-precision)"))
  ;[1 1 1] Update Health
  (bind _output_get (set `self.CurrentHealth` (`KismetMathLibrary.FClamp` (+ Health (`self.CurrentHealth`)) 0.0 (`self.MaxHealth`))))
  (if (== _output_get 0.0)
    (set `self.IsDead` true)
    (`KismetSystemLibrary.K2_ClearAndInvalidateTimerHandle` (`self.Timer-RegenerationMP`))
    (`KismetSystemLibrary.K2_ClearAndInvalidateTimerHandle` (`self.Timer-RegenerationThirst`))
    (`KismetSystemLibrary.K2_ClearAndInvalidateTimerHandle` (`self.Timer-RegenerationHunger`))
    (`self.IsDeadDispatcher`)))

(event `-UpdateMP`
  (params (ManaPoints :type "Float (double-precision)"))
  ;[1 1 1] Update MP
  (bind _output_get (set `self.CurrentMP` (`KismetMathLibrary.FClamp` (+ ManaPoints (`self.CurrentMP`)) 0.0 (`self.MaxMP`))))
  (if (< _output_get (`self.MaxMP`))
    (if (and (not (`KismetSystemLibrary.K2_IsTimerActiveHandle` (`self.Timer-RegenerationMP`))) (not (`self.IsDead`)) (`self.RegenerationMP?`))
      (bind _returnvalue (`KismetSystemLibrary.K2_SetTimer` null "-RegenerationMP" (`self.SpeedRegenerationMP_InSeconds`) true))
      (set `self.Timer-RegenerationMP` _returnvalue))
    (else
      (`KismetSystemLibrary.K2_ClearAndInvalidateTimerHandle` (`self.Timer-RegenerationMP`)))))

(event `-UpdateStatsWidget`
  ;[1 1 1] Update Widget
  (bind _controller (`self.Controller`)
    (:`then`
      (bind (_success _pawn _playercontroller _storageref _inventoryopened _shiftpressed _ctrlpressed _isdead _mainwidget) (message `/Game/InventorySystem/Blueprints/Data/Interfaces/BPI_Interact.-InteractWithRef` _controller))
      (`/Engine/EditorBlueprintResources/StandardMacros.IsValid` _mainwidget
        (:`Is Valid`
          (`/Game/InventorySystem/Blueprints/UI/W_PlayerStats_Widget.-UpdateWidget` (`/Game/InventorySystem/Blueprints/UI/W_MainWidget.W_PlayerStats_Widget` _mainwidget)))))
    (:`else`)))

(event `-UpdateHunger`
  (params (HungerPoints :type "Float (double-precision)"))
  ;[1 1 1] Update Hunger
  (bind _output_get (set `self.CurrentHunger` (`KismetMathLibrary.FClamp` (+ HungerPoints (`self.CurrentHunger`)) 0.0 (`self.MaxHunger`))))
  (if (<= _output_get 0.0)
    (set `self.HungerIsOver` true)
    (`self.-UpdateHealth` (/ (`self.HungerTimerForPoint`) (/ -1.0 (`self.DamageHungerPerSecond`))))
    (else
      (set `self.HungerIsOver` false))))

(event `-UpdateThirst`
  (params (ThirstPoints :type "Float (double-precision)"))
  ;[1 1 1] Update Thirst
  (bind _output_get (set `self.CurrentThirst` (`KismetMathLibrary.FClamp` (+ ThirstPoints (`self.CurrentThirst`)) 0.0 (`self.MaxThirst`))))
  (if (<= _output_get 0.0)
    (set `self.ThirstIsOver` true)
    (`self.-UpdateHealth` (/ (`self.ThirstTimerForPoint`) (/ -1.0 (`self.DamageThirstPerSecond`))))
    (else
      (set `self.ThirstIsOver` false))))

(fn `-Init`
  (set `self.CurrentHealth` (`self.MaxHealth`))
  (set `self.CurrentMP` (`self.MaxMP`))
  (set `self.CurrentHunger` (`self.MaxHunger`))
  (set `self.CurrentThirst` (`self.MaxThirst`))
  (`self.-InitOwner`))

(fn `-RegenerationHunger`
  (`self.-UpdateHunger` -1.0))

(fn `-RegenerationMP`
  (`self.-UpdateMP` 1.0))

(fn `-RegenerationThirst`
  (`self.-UpdateThirst` -1.0))

(fn `-UpdateStats`
  (params (ItemStats :type "/Game/InventorySystem/Blueprints/Data/Structures/Str_ItemStats Structure (by ref)"))
  (bind (_health _mana _damage _hunger _thirst) (break `/Game/InventorySystem/Blueprints/Data/Structures/Str_ItemStats` ItemStats))
  (`self.-UpdateHealth` (`KismetMathLibrary.Conv_IntToDouble` _health))
  (`self.-UpdateHealth` (`KismetMathLibrary.Conv_IntToDouble` (* _damage -1)))
  (`self.-UpdateMP` (`KismetMathLibrary.Conv_IntToDouble` _mana))
  (`self.-UpdateHunger` (`KismetMathLibrary.Conv_IntToDouble` _hunger))
  (`self.-UpdateThirst` (`KismetMathLibrary.Conv_IntToDouble` _thirst)))

(fn `OnRep_CurrentHealth`
  (`self.-UpdateStatsWidget`))

(fn `OnRep_CurrentHunger`
  (`self.-UpdateStatsWidget`))

(fn `OnRep_CurrentMP`
  (`self.-UpdateStatsWidget`))

(fn `OnRep_CurrentThirst`
  (`self.-UpdateStatsWidget`))