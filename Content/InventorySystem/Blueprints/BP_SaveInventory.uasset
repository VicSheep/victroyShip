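; BP_SaveInventory holds saved inventory data as a SaveItemsInfo array, with each entry pairing a name with its items.
; FindSaveByPlayerName searches that array for the first entry matching the given name and stops there.
; It returns a success flag with the entry's index and items, or failure with index zero when no name matches.
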(fn `-FindSaveByPlayerName`
  (params (Name :type Text))
  (returns (Success :type Boolean) (Index :type Integer) (Items :type "Array of /Game/InventorySystem/Blueprints/Data/Structures/Str_Item Structure"))
  (locals (local_Success :type Boolean) (local_Items :type "Array of /Game/InventorySystem/Blueprints/Data/Structures/Str_Item Structure") (local_Index :type Integer))
  (for (_array_element _array_index) (`self.Save_Items_Info`)
    (bind (_name _items) (break `/Game/InventorySystem/Blueprints/Data/Structures/Str_SaveInfo` _array_element))
    (if (`KismetTextLibrary.EqualEqual_TextText` Name _name)
      (set `local.local_Success` true)
      (set `local.local_Items` _items)
      (set `local.local_Index` _array_index)
      (break)))
  (if (`local.local_Success`)
    (return true (`local.local_Index`) (`local.local_Items`))
    (else
      (return false 0))))