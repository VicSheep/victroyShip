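; Base world pickup actor for inventory items, showing name and amount labels from its class's item info.
; On overlap or interaction, it adds itself to the interacting player's storage via interface messages, and UseItem forwards its info to the controller.
; BP_PickUpActor animates collection; partial pickups spawn a ForAnim copy to fly while the original keeps the remainder.
; An optional looping timer spins the mesh, yaws labels toward the camera and distance-culls them.
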(event `self.ReceiveBeginPlay`
  ;[1 1 1] Init
  (bind _output_get (set `self.ItemInfo` (`.ItemInfo` (`/Game/InventorySystem/Blueprints/Data/Functions/BPFL_Functions.-GetItemInfo_Library` (`GameplayStatics.GetObjectClass` self)))))
  (`TextRenderComponent.K2_SetText` (`self.ItemName`) (`KismetTextLibrary.Conv_NameToText` (`.GameName_34_EF354188490A856216236DBA8A374DDE` (break `/Game/InventorySystem/Blueprints/Data/Structures/Str_ItemInfo` _output_get))))
  (`self.-UpdateAmount` (`self.Amount`))
  (if (`self.Rotation?`)
    (`self.-AddRotation`)
    (`KismetSystemLibrary.K2_SetTimer` null "-AddRotation" 0.04 true)))

(event `self.Sphere.OnComponentBeginOverlap`
  (params (OverlappedComponent :type "PrimitiveComponent Object Reference") (OtherActor :type "Actor Object Reference") (OtherComp :type "PrimitiveComponent Object Reference") (OtherBodyIndex :type Integer) (bFromSweep :type Boolean) (SweepResult :type "HitResult Structure (by ref)"))
  (`/Engine/EditorBlueprintResources/StandardMacros.IsValid` OtherActor
    (:`Is Valid`
      (if (not (`self.ForAnim`))
        (`self.-Interact` OtherActor)))))

(event `-Interact`
  (params (Target :type "Actor Object Reference"))
  ;[1 1 1] Interact
  (bind (_success _pawn _playercontroller _storageref _inventoryopened _shiftpressed _ctrlpressed _isdead) (message `/Game/InventorySystem/Blueprints/Data/Interfaces/BPI_Interact.-InteractWithRef` (`self.GetInstigatorController` Target)))
  (if (and _success (not _isdead))
    (set `self.InteractPawn` _pawn)
    (bind (_success_2 _index _rest) (message `/Game/InventorySystem/Blueprints/Data/Interfaces/BPI_Interact.-AddItemToStorage` _playercontroller _storageref (`GameplayStatics.GetObjectClass` self) (`self.Amount`) true))
    (if _success_2
      (if (== _rest 0)
        (`self.SetActorEnableCollision` false)
        (`|SpawnActorFromClass` "/Game/InventorySystem/Blueprints/BP_PickUpActor.BP_PickUpActor_C" (`KismetMathLibrary.MakeTransform` (`self.K2_GetActorLocation`) (struct :`Pitch` 90.0)) "AlwaysSpawn" "OverrideRootScale" null (`self.InteractPawn`) self null)
        (`SceneComponent.SetHiddenInGame` (`self.TextRender`) true false)
        (`SceneComponent.SetHiddenInGame` (`self.ItemName`) true false)
        (elif (!= (`self.Amount`) _rest)
          (bind _returnvalue (`|SpawnActorFromClass` (`GameplayStatics.GetObjectClass` self) (`self.GetTransform`) "AlwaysSpawn" "OverrideRootScale" null 1 true null))
          (`|SpawnActorFromClass` "/Game/InventorySystem/Blueprints/BP_PickUpActor.BP_PickUpActor_C" (`KismetMathLibrary.MakeTransform` (`self.K2_GetActorLocation`) (struct :`Pitch` 90.0)) "AlwaysSpawn" "OverrideRootScale" null (`self.InteractPawn`) _returnvalue null)
          (`self.SetActorEnableCollision` _returnvalue false)
          (`self.-UpdateAmount` _rest)
          (`SceneComponent.SetHiddenInGame` (`/Game/InventorySystem/Blueprints/Items/BP_Items_Master.TextRender` _returnvalue) true false)
          (`SceneComponent.SetHiddenInGame` (`/Game/InventorySystem/Blueprints/Items/BP_Items_Master.ItemName` _returnvalue) true false))))))

(event `-UpdateAmount`
  (params (Amount :type Integer))
  ;[1 1 1] Interact
  (set `self.Amount` Amount)
  (`self.-UpdateAmount_Multi`))

(event `-UpdateAmount_Multi`
  ;[1 1 1] Interact
  (`TextRenderComponent.K2_SetText` (`self.TextRender`) (`|FormatText` (`KismetTextLibrary.Conv_IntToText` (`self.Amount`) false false))))

(fn `-AddRotation`
  (bind _returnvalue (`GameplayStatics.GetPlayerController` 0))
  (bind (_returnvalue_roll _returnvalue_pitch _returnvalue_yaw) (`KismetMathLibrary.BreakRotator` (`KismetMathLibrary.FindLookAtRotation` (`self.K2_GetActorLocation`) (`PlayerCameraManager.GetCameraLocation` (`PlayerController.PlayerCameraManager` _returnvalue)))))
  (`SceneComponent.K2_AddRelativeRotation` (`self.StaticMesh`) (struct :`Yaw` 4.0) false false)
  (`/Engine/EditorBlueprintResources/StandardMacros.IsValid` _returnvalue
    (:`Is Valid`
      (`SceneComponent.K2_SetWorldRotation` (`self.TextRender`) (`KismetMathLibrary.MakeRotator` 0.0 0.0 _returnvalue_yaw) false false)
      (`SceneComponent.K2_SetWorldRotation` (`self.ItemName`) (`KismetMathLibrary.MakeRotator` 0.0 0.0 _returnvalue_yaw) false false)
      (if (<= (`self.GetDistanceTo` (`Controller.K2_GetPawn` _returnvalue)) 2000.0)
        (`SceneComponent.SetVisibility` (`self.ItemName`) true false)
        (`SceneComponent.SetVisibility` (`self.TextRender`) true false)
        (else
          (`SceneComponent.SetVisibility` (`self.ItemName`) false false)
          (`SceneComponent.SetVisibility` (`self.TextRender`) false false))))))

(fn `-SetItemInfo`
  (returns (Success :type Boolean) (ItemInfo :type "/Game/InventorySystem/Blueprints/Data/Structures/Str_ItemInfo Structure"))
  (locals (local_ItemFound :type Boolean) (local_ItemInfo :type "/Game/InventorySystem/Blueprints/Data/Structures/Str_ItemInfo Structure"))
  (bind _outrownames (`DataTableFunctionLibrary.GetDataTableRowNames` "/Game/InventorySystem/Blueprints/Data/DT/DT_Itemsinfo.DT_Itemsinfo"))
  (for _array_element _outrownames
    (bind _returnvalue (`|GetDataTableRow` "/Game/InventorySystem/Blueprints/Data/DT/DT_Itemsinfo.DT_Itemsinfo" _array_element)
      (:`then`
        (if (== (`GameplayStatics.GetObjectClass` self) (`.ItemClass_38_18B07B7A4542A642815C5CB9492C9AC4` (break `/Game/InventorySystem/Blueprints/Data/Structures/Str_ItemInfo` _returnvalue)))
          (set `local.local_ItemFound` true)
          (set `self.ItemInfo` _returnvalue)
          (break)))))
  (if (`local.local_ItemFound`)
    (return true (`local.local_ItemInfo`))
    (else
      (return false))))

(fn `-UseItem`
  (params (TargetPlayerController :type "PlayerController Object Reference"))
  (returns (Success :type Boolean))
  (message `/Game/InventorySystem/Blueprints/Data/Interfaces/BPI_Interact.-ItemUse` TargetPlayerController (`self.ItemInfo`))
  (return true))

(fn `UserConstructionScript`
  (`TextRenderComponent.K2_SetText` (`self.TextRender`) (`|FormatText` (`KismetTextLibrary.Conv_IntToText` (`self.Amount`) false false))))