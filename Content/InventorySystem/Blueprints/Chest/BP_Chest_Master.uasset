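; Master chest Blueprint that lets one player at a time open its storage component in the chest UI.
; Interacting marks it busy and binds the player's WChest widget to the storage and saved slot layout; the same player interacting again closes it.
; Tick frees the chest when that player moves out of range, saving slot positions and hiding the widget.
; Storage initialization is delayed on BeginPlay outside standalone play.
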(event `self.ReceiveBeginPlay`
  ;[1 1 1] Init
  (`KismetSystemLibrary.Delay` (select `bool` (`KismetSystemLibrary.IsStandalone`) :`false` 4.0 :!type "Float (single-precision)"))
  (`/Game/InventorySystem/Blueprints/Components/BP_Storage_Component.-Init` (`self.BP_Storage_Component`)))

(event `-Close_Multi`
  (bind _playercontrollerinteract (`self.PlayerControllerInteract`))
  ;[1 1 1] Close Multi
  (bind (_success _pawn _playercontroller _storageref _inventoryopened _shiftpressed _ctrlpressed _isdead _mainwidget) (message `/Game/InventorySystem/Blueprints/Data/Interfaces/BPI_Interact.-InteractWithRef` _playercontrollerinteract))
  (`/Engine/EditorBlueprintResources/StandardMacros.IsValid` _mainwidget
    (:`Is Valid`
      (`/Game/InventorySystem/Blueprints/UI/Chest/W_Chest.-Close` (`/Game/InventorySystem/Blueprints/UI/W_MainWidget.W_Chest` _mainwidget))
      (message `/Game/InventorySystem/Blueprints/Data/Interfaces/BPI_Interact.-OpenCloseInventory_Interface` _playercontrollerinteract true))))

(event `/Game/InventorySystem/Blueprints/Data/Interfaces/BPI_Interact.-Interact`
  (params (PlayerController :type "PlayerController Object Reference"))
  ;[1 1 1] Interact
  (if (not (`self.Busy`))
    (`self.-OpenChest` PlayerController)
    (else
      (bind _playercontrollerinteract (`self.PlayerControllerInteract`)
        (:`then`
          (if (== _playercontrollerinteract PlayerController)
            (`self.-Close_Multi`)))
        (:`else`)))))

(event `-OpenChest_Client`
  (params (PlayerControllerInteract :type "PlayerController Object Reference"))
  ;[1 1 1] Open Chest
  (bind _output_get (set `self.PlayerControllerInteract` PlayerControllerInteract))
  (bind (_success _pawn _playercontroller _storageref _inventoryopened _shiftpressed _ctrlpressed _isdead _mainwidget) (message `/Game/InventorySystem/Blueprints/Data/Interfaces/BPI_Interact.-InteractWithRef` _output_get))
  (if (not (`KismetSystemLibrary.IsDedicatedServer`))
    (`/Engine/EditorBlueprintResources/StandardMacros.IsValid` _mainwidget
      (:`Is Valid`
        (bind _w_chest (`/Game/InventorySystem/Blueprints/UI/W_MainWidget.W_Chest` _mainwidget))
        (set `/Game/InventorySystem/Blueprints/UI/Chest/W_Chest.ChestRef` self _w_chest)
        (set `/Game/InventorySystem/Blueprints/UI/Chest/W_Chest.InteractOwnerController` (`self.PlayerControllerInteract`) _w_chest)
        (if (not (`Widget.IsVisible` _w_chest))
          (set `/Game/InventorySystem/Blueprints/UI/Chest/W_Chest.StorageComponentRef` (`self.BP_Storage_Component`) _w_chest)
          (`/Game/InventorySystem/Blueprints/UI/Chest/W_Chest.-UpdateStorageGrid` _w_chest (`/Game/InventorySystem/Blueprints/Components/BP_Storage_Component.SavedSlotsPositions` (`self.BP_Storage_Component`)))
          (`Widget.SetVisibility` _w_chest "Visible"))))))

(event `-OpenChest`
  (params (PlayerControllerInteract :type "PlayerController Object Reference"))
  ;[1 1 1] Open Chest
  (set `self.Busy` true)
  (`self.-OpenChest_Client` PlayerControllerInteract))

(event `self.ReceiveTick`
  (params (DeltaSeconds :type "Float (single-precision)"))
  ;[1 1 1] Distance to Close Chest
  (bind _playercontrollerinteract (`self.PlayerControllerInteract`)
    (:`then`
      (if (>= (`self.GetDistanceTo` (`Controller.K2_GetPawn` _playercontrollerinteract)) 300.0)
        (set `self.Busy` false)
        (bind (_success _pawn _playercontroller _storageref _inventoryopened _shiftpressed _ctrlpressed _isdead _mainwidget) (message `/Game/InventorySystem/Blueprints/Data/Interfaces/BPI_Interact.-InteractWithRef` _playercontrollerinteract))
        (`/Engine/EditorBlueprintResources/StandardMacros.IsValid` _mainwidget
          (:`Is Valid`
            (bind _w_chest (`/Game/InventorySystem/Blueprints/UI/W_MainWidget.W_Chest` _mainwidget))
            (bind _savedpositionslots (`/Game/InventorySystem/Blueprints/UI/Chest/W_Chest.-SaveSlotsPositions` _w_chest))
            (set `/Game/InventorySystem/Blueprints/Components/BP_Storage_Component.SavedSlotsPositions` _savedpositionslots (`self.BP_Storage_Component`))
            (`Widget.SetVisibility` _w_chest "Hidden")
            (set `self.PlayerControllerInteract` null)))))
    (:`else`)))

(fn `-AddItemToStorage`
  (params (TargetStorage :type "/Game/InventorySystem/Blueprints/Components/BP_Storage_Component Object Reference") (Item :type "/Game/InventorySystem/Blueprints/Items/BP_Items_Master Class Reference") (Amount :type Integer) (`UpdateInvetory?` :type Boolean))
  (returns (Success :type Boolean) (Index :type Integer) (Rest :type Integer) (AddedItems :type Integer))
  (return false 0 0 0))

(fn `-GetInfoToInteract`
  (returns (Success :type Boolean) (ActorRef :type "Actor Object Reference") (Busy :type Boolean))
  (return true self (`self.Busy`)))

(fn `-Init_Start_Items`
  (`/Game/InventorySystem/Blueprints/Components/BP_Storage_Component.-Init_Items` (`self.BP_Storage_Component`)))

(fn `-InteractWithRef`
  (returns (Success :type Boolean) (Pawn :type "Pawn Object Reference") (PlayerController :type "PlayerController Object Reference") (StorageRef :type "/Game/InventorySystem/Blueprints/Components/BP_Storage_Component Object Reference") (InventoryOpened :type Boolean) (ShiftPressed :type Boolean) (CtrlPressed :type Boolean) (IsDead :type Boolean) (MainWidget :type "/Game/InventorySystem/Blueprints/UI/W_MainWidget Object Reference"))
  (return false null null null false false false false null))

(fn `UserConstructionScript`)