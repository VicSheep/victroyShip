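; BP_PickUpActor is a helper actor that animates a picked-up item (StartTarget) flying to EndTarget, running only on authority.
; The first timeline moves the collision-disabled item along a runtime spline ending above EndTarget, adding a fresh spline component every update to follow the target.
; A second timeline lerps the item into EndTarget while shrinking it, then destroys the latest spline, the item and itself.
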(event `self.ReceiveBeginPlay`
  (`/Engine/EditorBlueprintResources/ActorMacros.Switch Has Authority`
    (:`Authority`
      (`self.-PickUpAnimation`))))

(event `-PickUpAnimation`
  (bind _starttarget (`self.StartTarget`))
  (`self.-PickUpItem`)
  (`self.SetActorEnableCollision` (`self.StartTarget`) false)
  (`TimelineComponent.SetPlayRate` (`self.TL_PickUp`) (`self.PlayRate`))
  (bind (_direction _newtrack_0) (`Timeline|TL_PickUp` :!via `PlayFromStart`)
    (:`Update`
      (`self.-PickUpItem`)
      (`self.K2_SetActorLocation` (`self.StartTarget`) (`SplineComponent.GetLocationAtTime` (`self.PickUpSpline`) (`KismetMathLibrary.Lerp` 0.0 1.0 _newtrack_0) "World" false) false true))
    (:`Finished`
      (set `self.LastLocation` (`self.K2_GetActorLocation` (`self.StartTarget`)))
      (bind (_direction_2 _newtrack_0_2) (`Timeline|TL_2` :!via `PlayFromStart`)
        (:`Update`
          (`self.K2_SetActorLocation` _starttarget (`KismetMathLibrary.VLerp` (`self.LastLocation`) (`self.K2_GetActorLocation` (`self.EndTarget`)) _newtrack_0_2) false false)
          (`self.SetActorScale3D` _starttarget (`KismetMathLibrary.VLerp` (1.0 1.0 1.0) (0.01 0.01 0.01) _newtrack_0_2)))
        (:`Finished`
          (`|ExecutionSequence`
            (:`then_0`
              (bind _pickupspline (`self.PickUpSpline`)
                (:`then`
                  (`ActorComponent.K2_DestroyComponent` _pickupspline))
                (:`else`)))
            (:`then_1`
              (`self.K2_DestroyActor` (`self.StartTarget`))
              (`self.K2_DestroyActor`))))))))

(fn `-PickUpItem`
  (bind _endtarget (`self.EndTarget`))
  (bind _returnvalue (`AddComponent|NODE_AddSplineComponent-2`))
  (set `self.PickUpSpline` _returnvalue)
  (`SplineComponent.AddSplinePoint` (`self.PickUpSpline`) (+ (`self.K2_GetActorLocation` _endtarget) (`KismetMathLibrary.MakeVector` 0.0 0.0 (+ (.z (`.BoxExtent` (`self.GetActorBounds` _endtarget true))) 20.0))) "World" true))

(fn `UserConstructionScript`)