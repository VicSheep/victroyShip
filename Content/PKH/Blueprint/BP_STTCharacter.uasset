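; Player character that adds push-to-talk voice recording and farming controls.
; Holding R, unless chatting, runs RecordComp and records the Record submix; release exports a WAV to TalkComp's path and calls its nearby-object check.
; F passes the nearest overlapping ground actor to FarmerComponent for farming interaction.
; T opens plant info when that ground has a plant, and I opens the tool widget.
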(event `Key|R`
  (params (Key :type "Key Structure"))
  (bind _talkcomp (`self.TalkComp`))
  (bind _recordcomp (`self.RecordComp`))
  ;[1 1 1] Comment
  (:`Pressed`
    (if (not (`TextInputComponent.IsChatting` (`self.ChatComp`)))
      (`SynthComponent.Start` _recordcomp)
      (`AudioMixerBlueprintLibrary.StartRecordingOutput` 0.0 "/Game/PKH/STT/Record.Record")
      (`KismetSystemLibrary.PrintString` "start")))
  (:`Released`
    (`SynthComponent.Stop` _recordcomp)
    (`AudioMixerBlueprintLibrary.StopRecordingOutput` "WavFile" (`TalkComponent.RecordFileName` _talkcomp) (`TalkComponent.RecordFileDir` _talkcomp) "/Game/PKH/STT/Record.Record" null)
    (`KismetSystemLibrary.PrintString` "end")
    (`TalkComponent.CheckNearbyObjects` (`self.TalkComp`))))

(event `Key|F`
  (params (Key :type "Key Structure"))
  (bind _farmercomponent (`self.FarmerComponent`))
  ;[1 1 1] 상호작용 키
  (:`Pressed`
    ;[1 1 1] 땅에 식물이 이미 심겨 있는지 확인
    (bind _asbp_ground_actor (cast `/Game/JIU/Blueprints/BP_GroundActor` (`.ReturnValue` (`GameplayStatics.FindNearestActor` (`self.K2_GetActorLocation`) (`self.GetOverlappingActors` "/Script/victroyShip.GroundActor")))))
    (`/Engine/EditorBlueprintResources/StandardMacros.IsValid` _asbp_ground_actor
      (:`Is Valid`
        (set `FarmerComponent.Ground` _asbp_ground_actor _farmercomponent)
        (`FarmerComponent.FarmingInteraction` _farmercomponent)))))

(event `Key|T`
  (params (Key :type "Key Structure"))
  ;[1 1 1] 식물 상태창
  (:`Pressed`
    ;[1 1 1] 땅에 식물이 이미 심겨 있는지 확인
    (bind _asbp_ground_actor (cast `/Game/JIU/Blueprints/BP_GroundActor` (`.ReturnValue` (`GameplayStatics.FindNearestActor` (`self.K2_GetActorLocation`) (`self.GetOverlappingActors` "/Script/victroyShip.GroundActor")))))
    (`/Engine/EditorBlueprintResources/StandardMacros.IsValid` (`GroundActor.Plant` _asbp_ground_actor)
      (:`Is Valid`
        (`FarmerComponent.OpenInfoWidget` (`self.FarmerComponent`))))))

(event `Key|I`
  (params (Key :type "Key Structure"))
  ;[1 1 1] 도구창
  (:`Pressed`
    (`FarmerComponent.OpenToolWidget` (`self.FarmerComponent`))))

(fn `UserConstructionScript`)