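; BP_TestPlayer is a test player Blueprint that records audio to a WAV file while the 1 key is held.
; Pressing the key starts RecordComp and begins recording output on the Record submix, and releasing it stops both and exports the result as TestWav.
; Print strings mark start and end, and the BeginPlay, overlap and Tick events are disabled stubs.
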(event `Key|One`
  (params (Key :type "Key Structure"))
  (bind _recordcomp (`self.RecordComp`))
  (:`Pressed`
    (`SynthComponent.Start` _recordcomp)
    (`AudioMixerBlueprintLibrary.StartRecordingOutput` 0.0 "/Game/PKH/STT/Record.Record")
    (`KismetSystemLibrary.PrintString` "Start"))
  (:`Released`
    (`SynthComponent.Stop` _recordcomp)
    (`AudioMixerBlueprintLibrary.StopRecordingOutput` "WavFile" "TestWav" "" "/Game/PKH/STT/Record.Record" null)
    (`KismetSystemLibrary.PrintString` "End")))

(fn `UserConstructionScript`
  (`parent.UserConstructionScript`))