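; Farm-life player character, apparently a backup copy, handling hotbar selection, inventory and storage screens, item dropping and stamina-restoring food.
; The mouse wheel cycles ten slots, E toggles inventory, and debug keys grant items or stamina.
; V line-traces from the camera; non-interactable results lead to a consumable check, whose true return is unwired, so eating never starts.
; Consume repeats after a delay while right mouse is held, adding stamina and decrementing the stack.
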(event `InputAxis|MW`
  (params (AxisValue :type "Float (single-precision)"))
  (bind _selectedslot (`self.SelectedSlot`))
  (`|ExecutionSequence`
    (:`then_0`
      (set `self.SelectedSlot` (`KismetMathLibrary.FTrunc` (+ (`self.SelectedSlot`) AxisValue)))
      (if (> _selectedslot 9)
        (set `self.SelectedSlot` 0)
        (elif (< _selectedslot 0)
          (set `self.SelectedSlot` 9))))
    (:`then_1`
      (`self.UpdateSelectedSlot`))))

(event `Key|V`
  (params (Key :type "Key Structure"))
  (:`Pressed`
    (`self.Interact`)))

(event `Key|C`
  (params (Key :type "Key Structure"))
  (:`Pressed`
    (if (> (`self.barStaminaCurn`) (`self.barStaminaMax`))
      (`KismetSystemLibrary.PrintString` "MaxStanina")
      (else
        (bind _output_get (set `self.barStaminaCurn` (+ (`self.barStaminaCurn`) 1.0)))
        (`KismetSystemLibrary.PrintString` (`KismetStringLibrary.Conv_DoubleToString` _output_get))))))

(event `Key|E`
  (params (Key :type "Key Structure"))
  (:`Pressed`
    (`self.ToggleInventory`)))

(event `Key|Q`
  (params (Key :type "Key Structure"))
  (:`Pressed`
    (`/Game/OJS/BaseInventorySystem/BPC_InventoryCompBase.SetItemInfoAtIndex` (`self.BPC_InventoryCompBase`) 0 "/Game/OJS/BaseInventorySystem/Items/BP_ItemStone.BP_ItemStone_C" 1)
    (`/Game/OJS/BaseInventorySystem/BPC_InventoryCompBase.SetItemInfoAtIndex` (`self.BPC_InventoryCompBase`) 1 "/Game/OJS/BaseInventorySystem/Items/BP_ItemWood.BP_ItemWood_C" 16)
    (`/Game/OJS/BaseInventorySystem/BPC_InventoryCompBase.SetItemInfoAtIndex` (`self.BPC_InventoryCompBase`) 2 "/Game/OJS/BaseInventorySystem/Items/BP_ItemWood.BP_ItemWood_C" 8)
    (`/Game/OJS/BaseInventorySystem/BPC_InventoryCompBase.SetItemInfoAtIndex` (`self.BPC_InventoryCompBase`) 3 "/Game/OJS/BaseInventorySystem/Items/BP_ItemStone.BP_ItemStone_C" 1)
    (`/Game/OJS/BaseInventorySystem/BPC_InventoryCompBase.SetItemInfoAtIndex` (`self.BPC_InventoryCompBase`) 4 "/Game/OJS/BaseInventorySystem/Items/BP_ItemEat.BP_ItemEat_C" 5)
    (`KismetSystemLibrary.PrintString` "cheet")))

(event `Key|RightMouseButton`
  (params (Key :type "Key Structure"))
  (:`Pressed`
    (set `self.RMB` true))
  (:`Released`
    (set `self.RMB` false)))

(event `Consume`
  (bind _ab1 (`self.AB1`))
  (bind _selectedslot (`self.SelectedSlot`))
  (bind (_item _quantity) (`/Game/OJS/BaseInventorySystem/BPC_InventoryCompBase.GetItemInfoAtIndex` _ab1 _selectedslot))
  ;[1 1 1] Consum Items
  (bind _asbp_master_consumable (castclass `/Game/OJS/BaseInventorySystem/Items/BP_MasterConsumable` (`/Game/OJS/BaseInventorySystem/BPC_InventoryCompBase.GetItemInfoAtIndex` (`self.AB1`) (`self.SelectedSlot`))))
  (`KismetSystemLibrary.Delay` 1.0)
  (if (`self.RMB`)
    (if (> (`self.barStaminaCurn`) (`self.barStaminaMax`))
      (`KismetSystemLibrary.PrintString` "MaxStanina")
      (else
        (bind _output_get (set `self.barStaminaCurn` (+ (`self.barStaminaCurn`) (defaults `Object` _asbp_master_consumable))))
        (`KismetSystemLibrary.PrintString` (`KismetStringLibrary.Conv_DoubleToString` _output_get))
        (`/Game/OJS/BaseInventorySystem/BPC_InventoryCompBase.SetItemInfoAtIndex` _ab1 _selectedslot _item (- _quantity 1))
        (if (== _quantity 0)
          (`/Game/OJS/BaseInventorySystem/BPC_InventoryCompBase.SetItemInfoAtIndex` _ab1 _selectedslot null 0)
          (else
            (`self.Consume`)))))
    (else
      (`KismetSystemLibrary.PrintString` "can't eat"))))

(fn `DropItem`
  (params (ItemToDrop :type "/Game/OJS/BaseInventorySystem/BP_MasterItem Class Reference") (QuantityToDrop :type Integer))
  (locals (LocalItemToDrop :type "/Game/OJS/BaseInventorySystem/BP_MasterItem Class Reference") (LocalQuantityToDrop :type Integer))
  (bind _followcamera (`self.FollowCamera`))
  (set `local.LocalItemToDrop` ItemToDrop)
  (set `local.LocalQuantityToDrop` QuantityToDrop)
  (`|SpawnActorFromClass` "/Game/OJS/BaseInventorySystem/BP_MasterPickupActor.BP_MasterPickupActor_C" (`KismetMathLibrary.MakeTransform` (+ (`SceneComponent.K2_GetComponentLocation` _followcamera) (* (`KismetMathLibrary.GetForwardVector` (`SceneComponent.K2_GetComponentRotation` _followcamera)) 666.0))) "Undefined" "MultiplyWithRoot" null (`local.LocalItemToDrop`) (`local.LocalQuantityToDrop`) self null))

(fn `HoldingConsumableItem?`
  (returns (True :type Boolean))
  (switch `/Game/OJS/BaseInventorySystem/StructsAndEnums/ItemCategory` (`.ItemCategory` (defaults `Object` (`/Game/OJS/BaseInventorySystem/BPC_InventoryCompBase.GetItemInfoAtIndex` (`self.AB1`) (`self.SelectedSlot`))))
    (:`NewEnumerator0`
      (return false))))

(fn `Interact`
  (bind _followcamera (`self.FollowCamera`))
  (bind _returnvalue (`SceneComponent.K2_GetComponentLocation` _followcamera))
  (bind _outhit (`KismetSystemLibrary.LineTraceSingle` :`Start` _returnvalue :`End` (+ _returnvalue (* (`KismetMathLibrary.GetForwardVector` (`SceneComponent.K2_GetComponentRotation` _followcamera)) 600.0)) :`TraceChannel` "TraceTypeQuery1" :`DrawDebugType` "ForDuration" :`DrawTime` 1.0))
  (if (`KismetSystemLibrary.DoesImplementInterface` (`.HitActor` (`GameplayStatics.BreakHitResult` _outhit)) "/Game/OJS/BaseInventorySystem/Interface/InteractInterface.InteractInterface_C")
    _
    (elif (`self.HoldingConsumableItem?`)
      (`self.Consume`))))

(fn `ToggleInventory`
  (bind _returnvalue (`GameplayStatics.GetPlayerController` 0))
  (switch `ESlateVisibility` (`Widget.GetVisibility` (`/Game/OJS/BaseInventorySystem/WBP_FLdHUD.PlayerInventory` (`self.HudRef`)))
    (:`Visible`
      (`Widget.SetVisibility` (`/Game/OJS/BaseInventorySystem/WBP_FLdHUD.PlayerInventory` (`self.HudRef`)) "Hidden")
      (`WidgetBlueprintLibrary.SetInputMode_GameOnly` _returnvalue)
      (set `PlayerController.bShowMouseCursor` false _returnvalue))
    (:`Hidden`
      (`Widget.SetVisibility` (`/Game/OJS/BaseInventorySystem/WBP_FLdHUD.PlayerInventory` (`self.HudRef`)) "Visible")
      (`WidgetBlueprintLibrary.SetInputMode_GameAndUIEx` _returnvalue null)
      (set `PlayerController.bShowMouseCursor` true _returnvalue)))
  (`WidgetSwitcher.SetActiveWidgetIndex` (`/Game/OJS/BaseInventorySystem/Interface/WBP_FLdIventoryWidget.WidgetSwitcher_55` (`/Game/OJS/BaseInventorySystem/WBP_FLdHUD.PlayerInventory` (`self.HudRef`))) 0))

(fn `ToggleStorage`
  (bind _returnvalue (`GameplayStatics.GetPlayerController` 0))
  (switch `ESlateVisibility` (`Widget.GetVisibility` (`/Game/OJS/BaseInventorySystem/WBP_FLdHUD.PlayerInventory` (`self.HudRef`)))
    (:`Visible`
      (`Widget.SetVisibility` (`/Game/OJS/BaseInventorySystem/WBP_FLdHUD.PlayerInventory` (`self.HudRef`)) "Hidden")
      (`WidgetBlueprintLibrary.SetInputMode_GameOnly` _returnvalue)
      (set `PlayerController.bShowMouseCursor` false _returnvalue))
    (:`Hidden`
      (`Widget.SetVisibility` (`/Game/OJS/BaseInventorySystem/WBP_FLdHUD.PlayerInventory` (`self.HudRef`)) "Visible")
      (`WidgetBlueprintLibrary.SetInputMode_GameAndUIEx` _returnvalue null)
      (set `PlayerController.bShowMouseCursor` true _returnvalue)))
  (`WidgetSwitcher.SetActiveWidgetIndex` (`/Game/OJS/BaseInventorySystem/Interface/WBP_FLdIventoryWidget.WidgetSwitcher_55` (`/Game/OJS/BaseInventorySystem/WBP_FLdHUD.PlayerInventory` (`self.HudRef`))) 1))

(fn `UpdateSelectedSlot`
  (for _array_element (`/Game/OJS/BaseInventorySystem/BPC_InventoryCompBase.SlotRef` (`self.AB1`))
    (`/Engine/EditorBlueprintResources/StandardMacros.IsValid` _array_element
      (:`Is Valid`
        (`/Game/OJS/BaseInventorySystem/Interface/WBP_FLdInventoryWidgetSlot.UpdateSelectedSlot` _array_element (`self.SelectedSlot`))))))

(fn `UserConstructionScript`)