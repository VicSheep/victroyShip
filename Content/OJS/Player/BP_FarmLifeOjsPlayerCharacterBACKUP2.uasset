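; Backup Blueprint of the farm-life player character, handling hotbar selection, inventory UI and farming actions.
; G checks the selected item's category and runs the matching tool or seed action on the nearest overlapping GroundActor, decrementing fertilizer and seeds.
; Other keys drive plant info, chat, WAV voice recording followed by a TalkComp nearby-object check, and a debug item cheat.
; Interact-box trace and stamina-eating logic are disconnected.
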(event `InputAxis|MW`
  (params (AxisValue :type "Float (single-precision)"))
  (bind _selectedslot (`self.SelectedSlot`))
  (`|ExecutionSequence`
    (:`then_0`
      (set `self.SelectedSlot` (`KismetMathLibrary.FTrunc` (+ (`self.SelectedSlot`) AxisValue)))
      (if (> _selectedslot 9)
        (set `self.SelectedSlot` 0)
        (elif (< _selectedslot 0)
          (set `self.SelectedSlot` 9))))
    (:`then_1`
      (`self.UpdateSelectedSlot`))))

(event `Key|V`
  (params (Key :type "Key Structure"))
  (:`Pressed`
    (`self.Interact_box`)))

(event `Key|C`
  (params (Key :type "Key Structure")))

(event `Key|E`
  (params (Key :type "Key Structure"))
  (:`Pressed`
    (`self.ToggleInventory`)))

(event `Key|G`
  (params (Key :type "Key Structure"))
  (:`Pressed`
    (`self.Interact_farm`)))

(event `Key|RightMouseButton`
  (params (Key :type "Key Structure")))

(event `Key|Q`
  (params (Key :type "Key Structure"))
  (:`Pressed`
    (`/Game/OJS/BaseInventorySystem/BPC_InventoryCompBase.SetItemInfoAtIndex` (`self.BPC_InventoryCompBase`) 0 "/Game/OJS/BaseInventorySystem/NewTool/BP_HoeItem.BP_HoeItem_C" 1)
    (`/Game/OJS/BaseInventorySystem/BPC_InventoryCompBase.SetItemInfoAtIndex` (`self.BPC_InventoryCompBase`) 1 "/Game/OJS/BaseInventorySystem/NewTool/BP_SickleItem.BP_SickleItem_C" 1)
    (`/Game/OJS/BaseInventorySystem/BPC_InventoryCompBase.SetItemInfoAtIndex` (`self.BPC_InventoryCompBase`) 2 "/Game/OJS/BaseInventorySystem/NewTool/BP_WateringItem.BP_WateringItem_C" 1)
    (`/Game/OJS/BaseInventorySystem/BPC_InventoryCompBase.SetItemInfoAtIndex` (`self.BPC_InventoryCompBase`) 3 "/Game/OJS/BaseInventorySystem/NewTool/BP_AxeItem.BP_AxeItem_C" 1)
    (`/Game/OJS/BaseInventorySystem/BPC_InventoryCompBase.SetItemInfoAtIndex` (`self.BPC_InventoryCompBase`) 4 "/Game/OJS/BaseInventorySystem/NewTool/BP_FertilizerItem.BP_FertilizerItem_C" 99)
    (`/Game/OJS/BaseInventorySystem/BPC_InventoryCompBase.SetItemInfoAtIndex` (`self.BPC_InventoryCompBase`) 9 "/Game/OJS/BaseInventorySystem/SEED/Seed1_Grape.Seed1_Grape_C" 1)
    (`/Game/OJS/BaseInventorySystem/BPC_InventoryCompBase.SetItemInfoAtIndex` (`self.BPC_InventoryCompBase`) 10 "/Game/OJS/BaseInventorySystem/SEED/Seed2_Cacao.Seed2_Cacao_C" 1)
    (`/Game/OJS/BaseInventorySystem/BPC_InventoryCompBase.SetItemInfoAtIndex` (`self.BPC_InventoryCompBase`) 11 "/Game/OJS/BaseInventorySystem/SEED/Seed3_Cauliflower.Seed3_Cauliflower_C" 1)
    (`/Game/OJS/BaseInventorySystem/BPC_InventoryCompBase.SetItemInfoAtIndex` (`self.BPC_InventoryCompBase`) 12 "/Game/OJS/BaseInventorySystem/SEED/Seed4_Strawberry.Seed4_Strawberry_C" 1)
    (`/Game/OJS/BaseInventorySystem/BPC_InventoryCompBase.SetItemInfoAtIndex` (`self.BPC_InventoryCompBase`) 13 "/Game/OJS/BaseInventorySystem/SEED/Seed5_Watermelon.Seed5_Watermelon_C" 1)
    (`KismetSystemLibrary.PrintString` "cheat")))

(event `Consume`
  ;[1 1 1] Consum Items
)

(event `Key|R`
  (params (Key :type "Key Structure"))
  (bind _talk_comp (`self.Talk Comp`))
  (bind _record_comp (`self.Record Comp`))
  (:`Pressed`
    (if (not (`TextInputComponent.IsChatting` (`self.Chat Comp`)))
      (`SynthComponent.Start` _record_comp)
      (`AudioMixerBlueprintLibrary.StartRecordingOutput` 0.0 "/Game/PKH/STT/Record.Record")
      (`KismetSystemLibrary.PrintString` "start")))
  (:`Released`
    (`SynthComponent.Stop` _record_comp)
    (`AudioMixerBlueprintLibrary.StopRecordingOutput` "WavFile" (`TalkComponent.RecordFileName` _talk_comp) (`TalkComponent.RecordFileDir` _talk_comp) "/Game/PKH/STT/Record.Record" null)
    (`KismetSystemLibrary.PrintString` "end")
    (`TalkComponent.CheckNearbyObjects` (`self.Talk Comp`))))

(event `Hoe`
  (`|ExecutionSequence`
    (:`then_0`
      (`KismetSystemLibrary.PrintString` "HoeExcute"))
    (:`then_1`
      (bind _asbp_ground_actor (cast `/Game/JIU/Blueprints/BP_GroundActor` (`.ReturnValue` (`GameplayStatics.FindNearestActor` (`self.K2_GetActorLocation`) (`self.GetOverlappingActors` "/Script/victroyShip.GroundActor")))))
      (`/Engine/EditorBlueprintResources/StandardMacros.IsValid` _asbp_ground_actor
        (:`Is Valid`
          (bind _output_get (set `self.As BP Ground Actor` _asbp_ground_actor))
          (`GroundActor.ProwGround` _output_get))))))

(event `Key|Enter`
  (params (Key :type "Key Structure"))
  (:`Pressed`
    (`TextInputComponent.Chat` (`self.Chat Comp`))))

(event `Key|Eight`
  (params (Key :type "Key Structure"))
  (:`Pressed`
    (`KismetSystemLibrary.PrintString` (`KismetStringLibrary.Conv_DoubleToString` (`GameplayStatics.GetGlobalTimeDilation`)))))

(event `Sickle`
  (`|ExecutionSequence`
    (:`then_0`
      (`KismetSystemLibrary.PrintString` "SickleExcute"))
    (:`then_1`
      (bind _asbp_ground_actor (cast `/Game/JIU/Blueprints/BP_GroundActor` (`.ReturnValue` (`GameplayStatics.FindNearestActor` (`self.K2_GetActorLocation`) (`self.GetOverlappingActors` "/Script/victroyShip.GroundActor")))))
      (`/Engine/EditorBlueprintResources/StandardMacros.IsValid` _asbp_ground_actor
        (:`Is Valid`
          (bind _output_get (set `self.As BP Ground Actor` _asbp_ground_actor))
          (`GroundActor.RemoveWeed` _output_get))))))

(event `Key|F`
  (params (Key :type "Key Structure"))
  ;[1 1 1] 식물 상태창
  (:`Pressed`
    ;[1 1 1] 땅에 식물이 이미 심겨 있는지 확인
    (bind _asbp_ground_actor (cast `/Game/JIU/Blueprints/BP_GroundActor` (`.ReturnValue` (`GameplayStatics.FindNearestActor` (`self.K2_GetActorLocation`) (`self.GetOverlappingActors` "/Script/victroyShip.GroundActor")))))
    (`/Engine/EditorBlueprintResources/StandardMacros.IsValid` (`GroundActor.Plant` _asbp_ground_actor)
      (:`Is Valid`
        (`FarmerComponent.OpenInfoWidget` (`self.Farmer`))))))

(event `Watering`
  (`|ExecutionSequence`
    (:`then_0`
      (`KismetSystemLibrary.PrintString` "WateringExcute"))
    (:`then_1`
      (bind _asbp_ground_actor (cast `/Game/JIU/Blueprints/BP_GroundActor` (`.ReturnValue` (`GameplayStatics.FindNearestActor` (`self.K2_GetActorLocation`) (`self.GetOverlappingActors` "/Script/victroyShip.GroundActor")))))
      (`/Engine/EditorBlueprintResources/StandardMacros.IsValid` _asbp_ground_actor
        (:`Is Valid`
          (bind _output_get (set `self.As BP Ground Actor` _asbp_ground_actor))
          (`GroundActor.WaterPlant` _output_get))))))

(event `Fertilizer`
  (bind _ab1 (`self.AB1`))
  (bind _selectedslot (`self.SelectedSlot`))
  (bind (_item _quantity) (`/Game/OJS/BaseInventorySystem/BPC_InventoryCompBase.GetItemInfoAtIndex` _ab1 _selectedslot))
  (bind _asbp_ground_actor (cast `/Game/JIU/Blueprints/BP_GroundActor` (`.ReturnValue` (`GameplayStatics.FindNearestActor` (`self.K2_GetActorLocation`) (`self.GetOverlappingActors` "/Script/victroyShip.GroundActor")))))
  (`/Engine/EditorBlueprintResources/StandardMacros.IsValid` _asbp_ground_actor
    (:`Is Valid`
      (bind _output_get (set `self.As BP Ground Actor` _asbp_ground_actor))
      (`GroundActor.FertilizePlant` _output_get)
      (`/Game/OJS/BaseInventorySystem/BPC_InventoryCompBase.SetItemInfoAtIndex` _ab1 _selectedslot _item (- _quantity 1))
      (if (== _quantity 0)
        (`/Game/OJS/BaseInventorySystem/BPC_InventoryCompBase.SetItemInfoAtIndex` _ab1 _selectedslot null 0)
        (else
          (`KismetSystemLibrary.PrintString` "FertilizerExcute"))))))

(event `Axe`
  (`|ExecutionSequence`
    (:`then_0`
      (`KismetSystemLibrary.PrintString` "AxeExcute"))
    (:`then_1`
      (bind _asbp_ground_actor (cast `/Game/JIU/Blueprints/BP_GroundActor` (`.ReturnValue` (`GameplayStatics.FindNearestActor` (`self.K2_GetActorLocation`) (`self.GetOverlappingActors` "/Script/victroyShip.GroundActor")))))
      (`/Engine/EditorBlueprintResources/StandardMacros.IsValid` _asbp_ground_actor
        (:`Is Valid`
          (bind _output_get (set `self.As BP Ground Actor` _asbp_ground_actor))
          (`GroundActor.RemovePlant` _output_get))))))

(event `GrpadSeed`
  (bind _ab1 (`self.AB1`))
  (bind _selectedslot (`self.SelectedSlot`))
  (bind (_item _quantity) (`/Game/OJS/BaseInventorySystem/BPC_InventoryCompBase.GetItemInfoAtIndex` _ab1 _selectedslot))
  (bind _asbp_ground_actor (cast `/Game/JIU/Blueprints/BP_GroundActor` (`.ReturnValue` (`GameplayStatics.FindNearestActor` (`self.K2_GetActorLocation`) (`self.GetOverlappingActors` "/Script/victroyShip.GroundActor")))))
  (`/Engine/EditorBlueprintResources/StandardMacros.IsValid` _asbp_ground_actor
    (:`Is Valid`
      (bind _output_get (set `self.As BP Ground Actor` _asbp_ground_actor))
      (`GroundActor.PlantingSeed` _output_get 0)
      (set `FarmerComponent.Ground` _output_get (`self.Farmer`))
      (`/Game/OJS/BaseInventorySystem/BPC_InventoryCompBase.SetItemInfoAtIndex` _ab1 _selectedslot _item (- _quantity 1))
      (if (== _quantity 0)
        (`/Game/OJS/BaseInventorySystem/BPC_InventoryCompBase.SetItemInfoAtIndex` _ab1 _selectedslot null 0)
        (else
          (`KismetSystemLibrary.PrintString` "SeedUse"))))))

(event `CacaoSeed`
  (bind _ab1 (`self.AB1`))
  (bind _selectedslot (`self.SelectedSlot`))
  (bind (_item _quantity) (`/Game/OJS/BaseInventorySystem/BPC_InventoryCompBase.GetItemInfoAtIndex` _ab1 _selectedslot))
  (bind _asbp_ground_actor (cast `/Game/JIU/Blueprints/BP_GroundActor` (`.ReturnValue` (`GameplayStatics.FindNearestActor` (`self.K2_GetActorLocation`) (`self.GetOverlappingActors` "/Script/victroyShip.GroundActor")))))
  (`/Engine/EditorBlueprintResources/StandardMacros.IsValid` _asbp_ground_actor
    (:`Is Valid`
      (bind _output_get (set `self.As BP Ground Actor` _asbp_ground_actor))
      (`GroundActor.PlantingSeed` _output_get 1)
      (set `FarmerComponent.Ground` _output_get (`self.Farmer`))
      (`/Game/OJS/BaseInventorySystem/BPC_InventoryCompBase.SetItemInfoAtIndex` _ab1 _selectedslot _item (- _quantity 1))
      (if (== _quantity 0)
        (`/Game/OJS/BaseInventorySystem/BPC_InventoryCompBase.SetItemInfoAtIndex` _ab1 _selectedslot null 0)
        (else
          (`KismetSystemLibrary.PrintString` "SeedUse"))))))

(event `CauliflowerSeed`
  (bind _ab1 (`self.AB1`))
  (bind _selectedslot (`self.SelectedSlot`))
  (bind (_item _quantity) (`/Game/OJS/BaseInventorySystem/BPC_InventoryCompBase.GetItemInfoAtIndex` _ab1 _selectedslot))
  (bind _asbp_ground_actor (cast `/Game/JIU/Blueprints/BP_GroundActor` (`.ReturnValue` (`GameplayStatics.FindNearestActor` (`self.K2_GetActorLocation`) (`self.GetOverlappingActors` "/Script/victroyShip.GroundActor")))))
  (`/Engine/EditorBlueprintResources/StandardMacros.IsValid` _asbp_ground_actor
    (:`Is Valid`
      (bind _output_get (set `self.As BP Ground Actor` _asbp_ground_actor))
      (`GroundActor.PlantingSeed` _output_get 2)
      (set `FarmerComponent.Ground` _output_get (`self.Farmer`))
      (`/Game/OJS/BaseInventorySystem/BPC_InventoryCompBase.SetItemInfoAtIndex` _ab1 _selectedslot _item (- _quantity 1))
      (if (== _quantity 0)
        (`/Game/OJS/BaseInventorySystem/BPC_InventoryCompBase.SetItemInfoAtIndex` _ab1 _selectedslot null 0)
        (else
          (`KismetSystemLibrary.PrintString` "SeedUse"))))))

(event `StrawberrySeed`
  (bind _ab1 (`self.AB1`))
  (bind _selectedslot (`self.SelectedSlot`))
  (bind (_item _quantity) (`/Game/OJS/BaseInventorySystem/BPC_InventoryCompBase.GetItemInfoAtIndex` _ab1 _selectedslot))
  (bind _asbp_ground_actor (cast `/Game/JIU/Blueprints/BP_GroundActor` (`.ReturnValue` (`GameplayStatics.FindNearestActor` (`self.K2_GetActorLocation`) (`self.GetOverlappingActors` "/Script/victroyShip.GroundActor")))))
  (`/Engine/EditorBlueprintResources/StandardMacros.IsValid` _asbp_ground_actor
    (:`Is Valid`
      (bind _output_get (set `self.As BP Ground Actor` _asbp_ground_actor))
      (`GroundActor.PlantingSeed` _output_get 3)
      (set `FarmerComponent.Ground` _output_get (`self.Farmer`))
      (`/Game/OJS/BaseInventorySystem/BPC_InventoryCompBase.SetItemInfoAtIndex` _ab1 _selectedslot _item (- _quantity 1))
      (if (== _quantity 0)
        (`/Game/OJS/BaseInventorySystem/BPC_InventoryCompBase.SetItemInfoAtIndex` _ab1 _selectedslot null 0)
        (else
          (`KismetSystemLibrary.PrintString` "SeedUse"))))))

(event `WaterMelonSeed`
  (bind _ab1 (`self.AB1`))
  (bind _selectedslot (`self.SelectedSlot`))
  (bind (_item _quantity) (`/Game/OJS/BaseInventorySystem/BPC_InventoryCompBase.GetItemInfoAtIndex` _ab1 _selectedslot))
  (bind _asbp_ground_actor (cast `/Game/JIU/Blueprints/BP_GroundActor` (`.ReturnValue` (`GameplayStatics.FindNearestActor` (`self.K2_GetActorLocation`) (`self.GetOverlappingActors` "/Script/victroyShip.GroundActor")))))
  (`/Engine/EditorBlueprintResources/StandardMacros.IsValid` _asbp_ground_actor
    (:`Is Valid`
      (bind _output_get (set `self.As BP Ground Actor` _asbp_ground_actor))
      (`GroundActor.PlantingSeed` _output_get 4)
      (set `FarmerComponent.Ground` _output_get (`self.Farmer`))
      (`/Game/OJS/BaseInventorySystem/BPC_InventoryCompBase.SetItemInfoAtIndex` _ab1 _selectedslot _item (- _quantity 1))
      (if (== _quantity 0)
        (`/Game/OJS/BaseInventorySystem/BPC_InventoryCompBase.SetItemInfoAtIndex` _ab1 _selectedslot null 0)
        (else
          (`KismetSystemLibrary.PrintString` "SeedUse"))))))

(fn `DropItem`
  (params (ItemToDrop :type "/Game/OJS/BaseInventorySystem/BP_MasterItem Class Reference") (QuantityToDrop :type Integer))
  (locals (LocalItemToDrop :type "/Game/OJS/BaseInventorySystem/BP_MasterItem Class Reference") (LocalQuantityToDrop :type Integer))
  (bind _followcamera (`self.FollowCamera`))
  (set `local.LocalItemToDrop` ItemToDrop)
  (set `local.LocalQuantityToDrop` QuantityToDrop)
  (`|SpawnActorFromClass` "/Game/OJS/BaseInventorySystem/BP_MasterPickupActor.BP_MasterPickupActor_C" (`KismetMathLibrary.MakeTransform` (+ (`SceneComponent.K2_GetComponentLocation` _followcamera) (* (`KismetMathLibrary.GetForwardVector` (`SceneComponent.K2_GetComponentRotation` _followcamera)) 666.0))) "Undefined" "MultiplyWithRoot" null (`local.LocalItemToDrop`) (`local.LocalQuantityToDrop`) self null))

(fn `HoldingAxeItem?`
  (returns (True :type Boolean))
  (switch `/Game/OJS/BaseInventorySystem/StructsAndEnums/ItemCategory` (`.ItemCategory` (defaults `Object` (`/Game/OJS/BaseInventorySystem/BPC_InventoryCompBase.GetItemInfoAtIndex` (`self.AB1`) (`self.SelectedSlot`))))
    (:`NewEnumerator0`
      _)
    (:`NewEnumerator4`
      _)
    (:`NewEnumerator5`
      _)
    (:`NewEnumerator6`
      _)
    (:`NewEnumerator7`
      _)
    (:`NewEnumerator8`
      (return true))
    (:`NewEnumerator9`
      _)
    (:`NewEnumerator10`
      _)
    (:`NewEnumerator11`
      _)
    (:`NewEnumerator12`
      _)
    (:`NewEnumerator13`
      _))
  (return false))

(fn `HoldingCacaoSeed?`
  (returns (True :type Boolean))
  (switch `/Game/OJS/BaseInventorySystem/StructsAndEnums/ItemCategory` (`.ItemCategory` (defaults `Object` (`/Game/OJS/BaseInventorySystem/BPC_InventoryCompBase.GetItemInfoAtIndex` (`self.AB1`) (`self.SelectedSlot`))))
    (:`NewEnumerator0`
      _)
    (:`NewEnumerator4`
      _)
    (:`NewEnumerator5`
      _)
    (:`NewEnumerator6`
      _)
    (:`NewEnumerator7`
      _)
    (:`NewEnumerator8`
      _)
    (:`NewEnumerator9`
      _)
    (:`NewEnumerator10`
      (return true))
    (:`NewEnumerator11`
      _)
    (:`NewEnumerator12`
      _)
    (:`NewEnumerator13`
      _))
  (return false))

(fn `HoldingCauliflowerSeed?`
  (returns (True :type Boolean))
  (switch `/Game/OJS/BaseInventorySystem/StructsAndEnums/ItemCategory` (`.ItemCategory` (defaults `Object` (`/Game/OJS/BaseInventorySystem/BPC_InventoryCompBase.GetItemInfoAtIndex` (`self.AB1`) (`self.SelectedSlot`))))
    (:`NewEnumerator0`
      _)
    (:`NewEnumerator4`
      _)
    (:`NewEnumerator5`
      _)
    (:`NewEnumerator6`
      _)
    (:`NewEnumerator7`
      _)
    (:`NewEnumerator8`
      _)
    (:`NewEnumerator9`
      _)
    (:`NewEnumerator10`
      _)
    (:`NewEnumerator11`
      (return true))
    (:`NewEnumerator12`
      _)
    (:`NewEnumerator13`
      _))
  (return false))

(fn `HoldingFertilizerItem?`
  (returns (True :type Boolean))
  (switch `/Game/OJS/BaseInventorySystem/StructsAndEnums/ItemCategory` (`.ItemCategory` (defaults `Object` (`/Game/OJS/BaseInventorySystem/BPC_InventoryCompBase.GetItemInfoAtIndex` (`self.AB1`) (`self.SelectedSlot`))))
    (:`NewEnumerator0`
      _)
    (:`NewEnumerator4`
      _)
    (:`NewEnumerator5`
      _)
    (:`NewEnumerator6`
      _)
    (:`NewEnumerator7`
      (return true))
    (:`NewEnumerator8`
      _)
    (:`NewEnumerator9`
      _)
    (:`NewEnumerator10`
      _)
    (:`NewEnumerator11`
      _)
    (:`NewEnumerator12`
      _)
    (:`NewEnumerator13`
      _))
  (return false))

(fn `HoldingGrapeSeed?`
  (returns (True :type Boolean))
  (switch `/Game/OJS/BaseInventorySystem/StructsAndEnums/ItemCategory` (`.ItemCategory` (defaults `Object` (`/Game/OJS/BaseInventorySystem/BPC_InventoryCompBase.GetItemInfoAtIndex` (`self.AB1`) (`self.SelectedSlot`))))
    (:`NewEnumerator0`
      _)
    (:`NewEnumerator4`
      _)
    (:`NewEnumerator5`
      _)
    (:`NewEnumerator6`
      _)
    (:`NewEnumerator7`
      _)
    (:`NewEnumerator8`
      _)
    (:`NewEnumerator9`
      (return true))
    (:`NewEnumerator10`
      _)
    (:`NewEnumerator11`
      _)
    (:`NewEnumerator12`
      _)
    (:`NewEnumerator13`
      _))
  (return false))

(fn `HoldingHoeItem?`
  (returns (True :type Boolean))
  (switch `/Game/OJS/BaseInventorySystem/StructsAndEnums/ItemCategory` (`.ItemCategory` (defaults `Object` (`/Game/OJS/BaseInventorySystem/BPC_InventoryCompBase.GetItemInfoAtIndex` (`self.AB1`) (`self.SelectedSlot`))))
    (:`NewEnumerator0`
      _)
    (:`NewEnumerator4`
      (return true))
    (:`NewEnumerator5`
      _)
    (:`NewEnumerator6`
      _)
    (:`NewEnumerator7`
      _)
    (:`NewEnumerator8`
      _)
    (:`NewEnumerator9`
      _)
    (:`NewEnumerator10`
      _)
    (:`NewEnumerator11`
      _)
    (:`NewEnumerator12`
      _)
    (:`NewEnumerator13`
      _))
  (return false))

(fn `HoldingSickleItem?`
  (returns (True :type Boolean))
  (switch `/Game/OJS/BaseInventorySystem/StructsAndEnums/ItemCategory` (`.ItemCategory` (defaults `Object` (`/Game/OJS/BaseInventorySystem/BPC_InventoryCompBase.GetItemInfoAtIndex` (`self.AB1`) (`self.SelectedSlot`))))
    (:`NewEnumerator0`
      _)
    (:`NewEnumerator4`
      _)
    (:`NewEnumerator5`
      (return true))
    (:`NewEnumerator6`
      _)
    (:`NewEnumerator7`
      _)
    (:`NewEnumerator8`
      _)
    (:`NewEnumerator9`
      _)
    (:`NewEnumerator10`
      _)
    (:`NewEnumerator11`
      _)
    (:`NewEnumerator12`
      _)
    (:`NewEnumerator13`
      _))
  (return false))

(fn `HoldingStarwBerrySeed?`
  (returns (True :type Boolean))
  (switch `/Game/OJS/BaseInventorySystem/StructsAndEnums/ItemCategory` (`.ItemCategory` (defaults `Object` (`/Game/OJS/BaseInventorySystem/BPC_InventoryCompBase.GetItemInfoAtIndex` (`self.AB1`) (`self.SelectedSlot`))))
    (:`NewEnumerator0`
      _)
    (:`NewEnumerator4`
      _)
    (:`NewEnumerator5`
      _)
    (:`NewEnumerator6`
      _)
    (:`NewEnumerator7`
      _)
    (:`NewEnumerator8`
      _)
    (:`NewEnumerator9`
      _)
    (:`NewEnumerator10`
      _)
    (:`NewEnumerator11`
      _)
    (:`NewEnumerator12`
      (return true))
    (:`NewEnumerator13`
      _))
  (return false))

(fn `HoldingWateringItem?`
  (returns (True :type Boolean))
  (switch `/Game/OJS/BaseInventorySystem/StructsAndEnums/ItemCategory` (`.ItemCategory` (defaults `Object` (`/Game/OJS/BaseInventorySystem/BPC_InventoryCompBase.GetItemInfoAtIndex` (`self.AB1`) (`self.SelectedSlot`))))
    (:`NewEnumerator0`
      _)
    (:`NewEnumerator4`
      _)
    (:`NewEnumerator5`
      _)
    (:`NewEnumerator6`
      (return true))
    (:`NewEnumerator7`
      _)
    (:`NewEnumerator8`
      _)
    (:`NewEnumerator9`
      _)
    (:`NewEnumerator10`
      _)
    (:`NewEnumerator11`
      _)
    (:`NewEnumerator12`
      _)
    (:`NewEnumerator13`
      _))
  (return false))

(fn `HoldingWaterMelonSeed?`
  (returns (True :type Boolean))
  (switch `/Game/OJS/BaseInventorySystem/StructsAndEnums/ItemCategory` (`.ItemCategory` (defaults `Object` (`/Game/OJS/BaseInventorySystem/BPC_InventoryCompBase.GetItemInfoAtIndex` (`self.AB1`) (`self.SelectedSlot`))))
    (:`NewEnumerator0`
      _)
    (:`NewEnumerator4`
      _)
    (:`NewEnumerator5`
      _)
    (:`NewEnumerator6`
      _)
    (:`NewEnumerator7`
      _)
    (:`NewEnumerator8`
      _)
    (:`NewEnumerator9`
      _)
    (:`NewEnumerator10`
      _)
    (:`NewEnumerator11`
      _)
    (:`NewEnumerator12`
      _)
    (:`NewEnumerator13`
      (return true)))
  (return false))

(fn `Interact_box`)

(fn `Interact_farm`
  (if (`self.HoldingHoeItem?`)
    (`self.Hoe` self)
    (elif (`self.HoldingSickleItem?`)
      (`self.Sickle` self)
      (elif (`self.HoldingWateringItem?`)
        (`self.Watering` self)
        (elif (`self.HoldingFertilizerItem?`)
          (`self.Fertilizer` self)
          (elif (`self.HoldingAxeItem?`)
            (`self.Axe` self)
            (elif (`self.HoldingGrapeSeed?`)
              (`self.GrpadSeed` self)
              (elif (`self.HoldingCacaoSeed?`)
                (`self.CacaoSeed` self)
                (elif (`self.HoldingCauliflowerSeed?`)
                  (`self.CauliflowerSeed` self)
                  (elif (`self.HoldingStarwBerrySeed?`)
                    (`self.StrawberrySeed` self)
                    (elif (`self.HoldingWaterMelonSeed?`)
                      (`self.WaterMelonSeed` self)
                      (else
                        (`KismetSystemLibrary.PrintString` "NONEITEM")))))))))))))

(fn `ToggleInventory`
  (bind _returnvalue (`GameplayStatics.GetPlayerController` 0))
  (switch `ESlateVisibility` (`Widget.GetVisibility` (`/Game/OJS/BaseInventorySystem/WBP_FLdHUD.PlayerInventory` (`self.HudRef`)))
    (:`Visible`
      (`Widget.SetVisibility` (`/Game/OJS/BaseInventorySystem/WBP_FLdHUD.PlayerInventory` (`self.HudRef`)) "Hidden")
      (`WidgetBlueprintLibrary.SetInputMode_GameOnly` _returnvalue)
      (set `PlayerController.bShowMouseCursor` false _returnvalue))
    (:`Hidden`
      (`Widget.SetVisibility` (`/Game/OJS/BaseInventorySystem/WBP_FLdHUD.PlayerInventory` (`self.HudRef`)) "Visible")
      (`WidgetBlueprintLibrary.SetInputMode_GameAndUIEx` _returnvalue null)
      (set `PlayerController.bShowMouseCursor` true _returnvalue)))
  (`WidgetSwitcher.SetActiveWidgetIndex` (`/Game/OJS/BaseInventorySystem/Interface/WBP_FLdIventoryWidget.WidgetSwitcher_55` (`/Game/OJS/BaseInventorySystem/WBP_FLdHUD.PlayerInventory` (`self.HudRef`))) 0))

(fn `ToggleStorage`
  (bind _returnvalue (`GameplayStatics.GetPlayerController` 0))
  (switch `ESlateVisibility` (`Widget.GetVisibility` (`/Game/OJS/BaseInventorySystem/WBP_FLdHUD.PlayerInventory` (`self.HudRef`)))
    (:`Visible`
      (`Widget.SetVisibility` (`/Game/OJS/BaseInventorySystem/WBP_FLdHUD.PlayerInventory` (`self.HudRef`)) "Hidden")
      (`WidgetBlueprintLibrary.SetInputMode_GameOnly` _returnvalue)
      (set `PlayerController.bShowMouseCursor` false _returnvalue))
    (:`Hidden`
      (`Widget.SetVisibility` (`/Game/OJS/BaseInventorySystem/WBP_FLdHUD.PlayerInventory` (`self.HudRef`)) "Visible")
      (`WidgetBlueprintLibrary.SetInputMode_GameAndUIEx` _returnvalue null)
      (set `PlayerController.bShowMouseCursor` true _returnvalue)))
  (`WidgetSwitcher.SetActiveWidgetIndex` (`/Game/OJS/BaseInventorySystem/Interface/WBP_FLdIventoryWidget.WidgetSwitcher_55` (`/Game/OJS/BaseInventorySystem/WBP_FLdHUD.PlayerInventory` (`self.HudRef`))) 1))

(fn `UpdateSelectedSlot`
  (for _array_element (`/Game/OJS/BaseInventorySystem/BPC_InventoryCompBase.SlotRef` (`self.AB1`))
    (`/Engine/EditorBlueprintResources/StandardMacros.IsValid` _array_element
      (:`Is Valid`
        (`/Game/OJS/BaseInventorySystem/Interface/WBP_FLdInventoryWidgetSlot.UpdateSelectedSlot` _array_element (`self.SelectedSlot`))))))

(fn `UserConstructionScript`)