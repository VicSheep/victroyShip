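; Player character Blueprint for a farm-life game that handles the inventory screen and item pickup.
; Tab toggles the lazily created inventory widget, switching cursor and input mode between UI and game.
; E ensures the widget exists, then passes overlapping item actors through the BPI_PickUp interface into the inventory component.
; Sphere overlaps set a range flag on any overlapping BP_FarmLifeOjsPlayerCharacter and print debug messages.
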(event `Key|Tab`
  (params (Key :type "Key Structure"))
  (bind _returnvalue (`GameplayStatics.GetPlayerController` 0))
  (:`Pressed`
    (`/Engine/EditorBlueprintResources/StandardMacros.FlipFlop`
      (:`A`
        (`self.InventoryWidget`
          (:`then`
            (`Widget.SetVisibility` (`self.InventoryWidget`) "Visible"))
          (:`else`
            (bind _returnvalue_2 (`|GenericCreateObject` (`GameplayStatics.GetPlayerController` 0) "/Game/OJS/UIs/WBP_FarmLifeOjsUserWidget.WBP_FarmLifeOjsUserWidget_C"))
            (bind _output_get (set `self.InventoryWidget` _returnvalue_2))
            (`UserWidget.AddToViewport` _output_get 0)))
        (`WidgetBlueprintLibrary.SetInputMode_GameAndUIEx` _returnvalue null)
        (set `PlayerController.bShowMouseCursor` true (`GameplayStatics.GetPlayerController` 0)))
      (:`B`
        (bind _inventorywidget (`self.InventoryWidget`)
          (:`then`
            (`Widget.SetVisibility` _inventorywidget "Hidden")
            (`WidgetBlueprintLibrary.SetInputMode_GameOnly` _returnvalue)
            (set `PlayerController.bShowMouseCursor` false _returnvalue))
          (:`else`))))))

(event `Key|E`
  (params (Key :type "Key Structure"))
  (:`Pressed`
    (`self.InventoryWidget`
      (:`then`
        _)
      (:`else`
        (bind _returnvalue (`|GenericCreateObject` "/Game/OJS/UIs/WBP_FarmLifeOjsUserWidget.WBP_FarmLifeOjsUserWidget_C"))
        (bind _output_get (set `self.InventoryWidget` _returnvalue))
        (`UserWidget.AddToViewport` _output_get 0)
        (`Widget.SetVisibility` (`self.InventoryWidget`) "Hidden")))
    (for _array_element (`self.GetOverlappingActors` "/Game/OJS/Items/BP_ItemActor1.BP_ItemActor1_C")
      (if (`KismetSystemLibrary.DoesImplementInterface` _array_element "/Game/OJS/Interfaces/BPI_PickUp.BPI_PickUp_C")
        (bind _item (message `/Game/OJS/Interfaces/BPI_PickUp.Pick Up Item` _array_element))
        (`/Game/OJS/Inventory/BPC_FLOPCInventory.Add Item To Inventory` (`self.BPC_FLOPCInventory`) _item)))))

(event `self.Sphere.OnComponentBeginOverlap`
  (params (OverlappedComponent :type "PrimitiveComponent Object Reference") (OtherActor :type "Actor Object Reference") (OtherComp :type "PrimitiveComponent Object Reference") (OtherBodyIndex :type Integer) (bFromSweep :type Boolean) (SweepResult :type "HitResult Structure (by ref)"))
  (bind _asbp_farm_life_ojs_player_character (cast `/Game/OJS/Player/BP_FarmLifeOjsPlayerCharacter` OtherActor))
  (set `/Game/OJS/Player/BP_FarmLifeOjsPlayerCharacter.RangeCheckBULL` true _asbp_farm_life_ojs_player_character)
  (`KismetSystemLibrary.PrintString` "rangeIN"))

(event `self.Sphere.OnComponentEndOverlap`
  (params (OverlappedComponent :type "PrimitiveComponent Object Reference") (OtherActor :type "Actor Object Reference") (OtherComp :type "PrimitiveComponent Object Reference") (OtherBodyIndex :type Integer))
  (bind _asbp_farm_life_ojs_player_character (cast `/Game/OJS/Player/BP_FarmLifeOjsPlayerCharacter` OtherActor))
  (set `/Game/OJS/Player/BP_FarmLifeOjsPlayerCharacter.RangeCheckBULL` false _asbp_farm_life_ojs_player_character)
  (`KismetSystemLibrary.PrintString` "rangeOUT"))

(fn `UserConstructionScript`)