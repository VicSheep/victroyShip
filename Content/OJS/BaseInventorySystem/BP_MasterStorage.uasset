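; BP_MasterStorage is an interactable storage actor that holds items in a BPCInventoryCompBase inventory component.
; Interact stores the player reference, has the HUD's PlayerInventory generate the storage view from that component, then calls ToggleStorage on the player and returns false.
; An unconnected chain in the event graph would seed farming tools and fertilizer after a delay, but it never runs.
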(event `self.ReceiveBeginPlay`)

(fn `Interact`
  (params (PlayerRef :type "/Game/OJS/Player/BP_FarmLifeOjsPlayerCharacter Object Reference"))
  (returns (Success :type Boolean))
  (set `self.Player Ref` PlayerRef)
  (`/Game/OJS/BaseInventorySystem/Interface/WBP_FLdIventoryWidget.GenerateStorageInventory` (`/Game/OJS/BaseInventorySystem/WBP_FLdHUD.PlayerInventory` (`/Game/OJS/Player/BP_FarmLifeOjsPlayerCharacter.HudRef` (`self.Player Ref`))) (`self.BPC_InventoryCompBase`))
  (`/Game/OJS/Player/BP_FarmLifeOjsPlayerCharacter.ToggleStorage` (`self.Player Ref`))
  (return false))

(fn `UserConstructionScript`)