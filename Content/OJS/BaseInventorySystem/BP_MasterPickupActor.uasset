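; Master pickup actor for a dropped inventory item, showing its mesh from the item class defaults and a popup with item and quantity.
; On BeginPlay it launches its sphere with an impulse built from the player's follow-camera location and forward vector, then destroys itself after five seconds.
; When the player character overlaps the sphere, it adds the item to their inventory, then destroys itself on success or keeps the remainder and refreshes the popup.
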(event `self.ReceiveBeginPlay`
  (bind _followcamera (`FarmLifeOjsPlayerCharacter.FollowCamera` (`self.PlayerRef`)))
  (bind _aswbp_pop_up_info (cast `/Game/OJS/BaseInventorySystem/WBP_PopUpInfo` (`WidgetComponent.GetWidget` (`self.PopupInfo`))))
  (set `self.As WBP Pop Up Info` _aswbp_pop_up_info)
  (`/Game/OJS/BaseInventorySystem/WBP_PopUpInfo.UpdateInfo` (`self.As WBP Pop Up Info`) (`self.Item`) (`self.Quantity`))
  (`PrimitiveComponent.AddImpulse` (`self.Sphere`) (+ (`SceneComponent.K2_GetComponentLocation` _followcamera) (* (`KismetMathLibrary.GetForwardVector` (`SceneComponent.K2_GetComponentRotation` _followcamera)) 25000.0)) "None" false)
  (`StaticMeshComponent.SetStaticMesh` (`self.StaticMesh`) (`.StaticMesh_25_A896D9364C90C184A4F79AA1522D5752` (break `/Game/OJS/BaseInventorySystem/StructsAndEnums/Iteminfo` (defaults `Object` (`self.Item`)))))
  (`KismetSystemLibrary.Delay` 5.0)
  (`self.K2_DestroyActor`))

(event `self.Sphere.OnComponentBeginOverlap`
  (params (OverlappedComponent :type "PrimitiveComponent Object Reference") (OtherActor :type "Actor Object Reference") (OtherComp :type "PrimitiveComponent Object Reference") (OtherBodyIndex :type Integer) (bFromSweep :type Boolean) (SweepResult :type "HitResult Structure (by ref)"))
  (bind _asbp_farm_life_ojs_player_character (cast `/Game/OJS/Player/BP_FarmLifeOjsPlayerCharacter` OtherActor))
  (bind (_success _remainder) (`/Game/OJS/BaseInventorySystem/BPC_InventoryCompBase.AddItem` (`/Game/OJS/Player/BP_FarmLifeOjsPlayerCharacter.BPC_InventoryCompBase` _asbp_farm_life_ojs_player_character) (`self.Item`) (`self.Quantity`)))
  (if _success
    (`self.K2_DestroyActor`)
    (else
      (set `self.Quantity` _remainder)
      (`/Game/OJS/BaseInventorySystem/WBP_PopUpInfo.UpdateInfo` (`self.As WBP Pop Up Info`) (`self.Item`) (`self.Quantity`)))))

(event `self.ReceiveTick`
  (params (DeltaSeconds :type "Float (single-precision)")))

(fn `UserConstructionScript`)