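; Drag-and-drop operation for inventory items that toggles the HUD's drop boxes while a usable item is being dragged.
; Dragged enables the drop boxes through the slot's HUD reference if the item class's default ItemInfo marks it Usable.
; Drop disables them under the same Usable check, while DragCancelled disables them unconditionally.
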(event `self.Dragged`
  (params (PointerEvent :type "PointerEvent Structure (by ref)"))
  (if (`.Usable?_20_4A0891074536744367F52C8D8EEB863E` (break `/Game/OJS/BaseInventorySystem/StructsAndEnums/Iteminfo` (defaults `Object` (`self.Item`))))
    (`/Game/OJS/BaseInventorySystem/WBP_FLdHUD.EnableDropboxs` (`/Game/OJS/BaseInventorySystem/Interface/WBP_FLdInventoryWidgetSlot.HudRef` (`self.SlotRef`)))))

(event `self.Drop`
  (params (PointerEvent :type "PointerEvent Structure (by ref)"))
  (if (`.Usable?_20_4A0891074536744367F52C8D8EEB863E` (break `/Game/OJS/BaseInventorySystem/StructsAndEnums/Iteminfo` (defaults `Object` (`self.Item`))))
    (`/Game/OJS/BaseInventorySystem/WBP_FLdHUD.DisableDropboxs` (`/Game/OJS/BaseInventorySystem/Interface/WBP_FLdInventoryWidgetSlot.HudRef` (`self.SlotRef`)))))

(event `self.DragCancelled`
  (params (PointerEvent :type "PointerEvent Structure (by ref)"))
  (`/Game/OJS/BaseInventorySystem/WBP_FLdHUD.DisableDropboxs` (`/Game/OJS/BaseInventorySystem/Interface/WBP_FLdInventoryWidgetSlot.HudRef` (`self.SlotRef`))))