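; Base inventory component that stores item classes and quantities in a Contents array sized to MaxSlots on BeginPlay.
; AddItem places items one unit at a time, topping up existing stacks below their max size before filling empty slots, and returns any remainder on failure.
; Stack rules come from each item class's default ItemInfo, and each slot write calls UpdateSlot on the matching SlotRef entry.
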(event `self.ReceiveBeginPlay`
  (`KismetArrayLibrary.Array_Resize` (`self.Contents`) (`self.MaxSlots`)))

(fn `AddItem`
  (params (Item :type "/Game/OJS/BaseInventorySystem/BP_MasterItem Class Reference") (Quantity :type Integer))
  (returns (Success :type Boolean) (Remainder :type Integer))
  (bind (_valid _index) (`self.ValidEmptySlot?`))
  (bind (_valid_2 _index_2) (`self.ValidStackableIndex?`))
  (bind (_valid_3 _index_3) (`self.ValidEmptySlot?`))
  (set `self.ItemToAdd` Item)
  (set `self.QuantityToAdd` Quantity)
  (if (`.Stackable?_16_5E05FBB84E2A305A02FDE080191C2604` (break `/Game/OJS/BaseInventorySystem/StructsAndEnums/Iteminfo` (defaults `Object` (`self.ItemToAdd`)))) :!label _label
    (if _valid_2
      (`self.AddOneToStackAtIndex` _index_2)
      (if (> (`self.QuantityToAdd`) 0)
        (goto _label)
        (else
          (return true 0)))
      (elif _valid
        (`self.AddOneAtIndex` _index)
        (if (> (`self.QuantityToAdd`) 0)
          (goto _label)
          (else
            (return true 0)))
        (else
          (return false (`self.QuantityToAdd`)))))
    (else
      ;[1 1 1] Handles non stackable items
      (if _valid_3 :!label _label_2
        (`self.AddOneAtIndex` _index_3)
        (if (> (`self.QuantityToAdd`) 0)
          (goto _label_2)
          (else
            (return true 0)))
        (else
          (return false (`self.QuantityToAdd`)))))))

(fn `AddOneAtIndex`
  (params (Index :type Integer))
  (locals (LocalIndex :type Integer))
  (bind _output_get (set `local.LocalIndex` Index))
  (`KismetArrayLibrary.Array_Set` (`self.Contents`) _output_get (make `/Game/OJS/BaseInventorySystem/StructsAndEnums/InventoryContents` (`self.ItemToAdd`) 1) true)
  (`/Game/OJS/BaseInventorySystem/Interface/WBP_FLdInventoryWidgetSlot.UpdateSlot` (`|GetArrayItem` (`self.SlotRef`) (`local.LocalIndex`)))
  (set `self.QuantityToAdd` (- (`self.QuantityToAdd`) 1))
  (return))

(fn `AddOneToStackAtIndex`
  (params (Index :type Integer))
  (locals (LocalIndex :type Integer))
  (bind (_output_item _output_quantity) (break `/Game/OJS/BaseInventorySystem/StructsAndEnums/InventoryContents` (`|GetArrayItem` (`self.Contents`) (`local.LocalIndex`))))
  (bind (_output_item_2 _output_quantity_2) (break `/Game/OJS/BaseInventorySystem/StructsAndEnums/InventoryContents` (`|GetArrayItem` (`self.Contents`) (`local.LocalIndex`))))
  (bind _output_get (set `local.LocalIndex` Index))
  (`KismetArrayLibrary.Array_Set` (`self.Contents`) _output_get (make `/Game/OJS/BaseInventorySystem/StructsAndEnums/InventoryContents` (`self.ItemToAdd`) (+ _output_quantity_2 1)) true)
  (if (<= _output_quantity 0)
    (`KismetArrayLibrary.Array_Set` (`self.Contents`) (`local.LocalIndex`) (make `/Game/OJS/BaseInventorySystem/StructsAndEnums/InventoryContents` null) true))
  (`/Game/OJS/BaseInventorySystem/Interface/WBP_FLdInventoryWidgetSlot.UpdateSlot` (`|GetArrayItem` (`self.SlotRef`) (`local.LocalIndex`)))
  (set `self.QuantityToAdd` (- (`self.QuantityToAdd`) 1))
  (return))

(fn `GetItemInfoAtIndex`
  (params (Index :type Integer))
  (returns (Item :type "/Game/OJS/BaseInventorySystem/BP_MasterItem Class Reference") (Quantity :type Integer))
  (locals (LocalIndex :type Integer))
  (bind (_output_item _output_quantity) (break `/Game/OJS/BaseInventorySystem/StructsAndEnums/InventoryContents` (`|GetArrayItem` (`self.Contents`) (`local.LocalIndex`))))
  (set `local.LocalIndex` Index)
  (return _output_item _output_quantity))

(fn `SetItemInfoAtIndex`
  (params (Index :type Integer) (Item :type "/Game/OJS/BaseInventorySystem/BP_MasterItem Class Reference") (Quantity :type Integer))
  (locals (LocalIndex :type Integer))
  (bind _output_get (set `local.LocalIndex` Index))
  (`KismetArrayLibrary.Array_Set` (`self.Contents`) _output_get (make `/Game/OJS/BaseInventorySystem/StructsAndEnums/InventoryContents` Item Quantity) true)
  (`/Game/OJS/BaseInventorySystem/Interface/WBP_FLdInventoryWidgetSlot.UpdateSlot` (`|GetArrayItem` (`self.SlotRef`) (`local.LocalIndex`)))
  (return))

(fn `ValidateInventorySlot`
  (params (Index :type Integer))
  (returns (Valid :type Boolean))
  (locals (LocalIndex :type Integer))
  (bind _output_item (break `/Game/OJS/BaseInventorySystem/StructsAndEnums/InventoryContents` (`|GetArrayItem` (`self.Contents`) (`local.LocalIndex`))))
  (set `local.LocalIndex` Index)
  (return (`KismetSystemLibrary.IsValidClass` _output_item)))

(fn `ValidEmptySlot?`
  (returns (Valid :type Boolean) (Index :type Integer))
  (for (_array_element _array_index) (`self.Contents`)
    (bind _returnvalue (not (`KismetSystemLibrary.IsValidClass` (`.Item_5_9928D6F248D944176D46429C89AA2089` (break `/Game/OJS/BaseInventorySystem/StructsAndEnums/InventoryContents` _array_element)))))
    (if _returnvalue
      (break)))
  (if _returnvalue
    (return true _array_index)
    (else
      (return false 0))))

(fn `ValidStackableIndex?`
  (returns (Valid :type Boolean) (Index :type Integer))
  (for (_array_element _array_index) (`self.Contents`)
    (bind (_item _quantity) (break `/Game/OJS/BaseInventorySystem/StructsAndEnums/InventoryContents` _array_element))
    (bind _returnvalue (and (== _item (`self.ItemToAdd`)) (< _quantity (`.MaxStackSize?_17_F4ADA25E405EB16E9F5056ABE149F026` (break `/Game/OJS/BaseInventorySystem/StructsAndEnums/Iteminfo` (defaults `Object` (`self.ItemToAdd`)))))))
    (if _returnvalue
      (break)))
  (if _returnvalue
    (return true _array_index)
    (else
      (return false 0))))