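; BP_ItemActor_Hoe is a world pickup that gives the player a hoe item.
; When the farm player character overlaps its Trigger, it adds one BP_HoeItem to the character's inventory component, then destroys itself on success or prints a failure message.
; Tick slowly spins the Model around its yaw axis.
; PickUpItem is empty, and older pickup and popup nodes remain disconnected.
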(event `self.Trigger.OnComponentBeginOverlap`
  (params (OverlappedComponent :type "PrimitiveComponent Object Reference") (OtherActor :type "Actor Object Reference") (OtherComp :type "PrimitiveComponent Object Reference") (OtherBodyIndex :type Integer) (bFromSweep :type Boolean) (SweepResult :type "HitResult Structure (by ref)"))
  (bind _asbp_farm_life_ojs_player_character (cast `/Game/OJS/Player/BP_FarmLifeOjsPlayerCharacter` OtherActor))
  (bind _success (`/Game/OJS/BaseInventorySystem/BPC_InventoryCompBase.AddItem` (`/Game/OJS/Player/BP_FarmLifeOjsPlayerCharacter.BPC_InventoryCompBase` _asbp_farm_life_ojs_player_character) "/Game/OJS/BaseInventorySystem/NewTool/BP_HoeItem.BP_HoeItem_C" 1))
  (if _success
    (`self.K2_DestroyActor`)
    (else
      (`KismetSystemLibrary.PrintString` "FAIL"))))

(event `self.ReceiveTick`
  (params (DeltaSeconds :type "Float (single-precision)"))
  (bind _model (`self.model`))
  (bind (_returnvalue_roll _returnvalue_pitch _returnvalue_yaw) (`KismetMathLibrary.BreakRotator` (`SceneComponent.K2_GetComponentRotation` _model)))
  (`SceneComponent.K2_SetWorldRotation` _model (`KismetMathLibrary.MakeRotator` _returnvalue_roll _returnvalue_pitch (+ _returnvalue_yaw (* DeltaSeconds 22.0))) false false))

(fn `Pick Up Item`
  (returns (item :type String)))

(fn `UserConstructionScript`)