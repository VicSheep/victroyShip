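; BP_outlineNameTest is a test actor with a name widget, used to toggle an outline effect and name labels together.
; On BeginPlay it finds the post-process volume tagged "outline", gathers all actors of its own class as NPCs, and sets its WB_Name text color.
; The O key drives a FlipFlop that sets the volume's Unbound flag and calls SetNameVisible on every gathered actor to show or hide names.
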(event `self.ReceiveBeginPlay`
  (bind _outactors (`GameplayStatics.GetAllActorsOfClassWithTag` "/Script/Engine.PostProcessVolume" "outline"))
  (for _array_element _outactors
    (set `self.outline postprocessvolume` _array_element))
  (bind _outactors_2 (`GameplayStatics.GetAllActorsOfClass` "BP_outlineNameTest_C"))
  (set `self.NPCs` _outactors_2)
  (bind _aswb_name (cast `/Game/LSH/outline/WB_Name` (`WidgetComponent.GetWidget` (`self.name`))))
  (`/Game/LSH/outline/WB_Name.SetTextColor` _aswb_name (`self.In Color and Opacity`)))

(event `Key|O`
  (params (Key :type "Key Structure"))
  (:`Pressed`
    (bind _isa (`/Engine/EditorBlueprintResources/StandardMacros.FlipFlop`)
      (:`A`
        _)
      (:`B`
        _))
    (set `PostProcessVolume.bUnbound` _isa (`self.outline postprocessvolume`))
    (for _array_element (`self.NPCs`)
      (`self.setNameVisible` _array_element _isa))))

(event `setNameVisible`
  (params (isVisible :type Boolean))
  (`SceneComponent.SetVisibility` (`self.name`) isVisible false))

(fn `UserConstructionScript`)